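; BP_Torch_02 is a torch prop with a point light that can optionally flicker.
; The construction script applies a configurable light intensity.
; When flickering is enabled, a random startup delay precedes a timeline that lerps the intensity between fixed bounds, overriding the configured value.
; A FlipFlop on the timeline's Finished output alternates reverse and forward playback to keep the flicker going.
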(event `self.ReceiveBeginPlay`
  ;[0 0 0] Flickering
  (if (`self.Flickering?`)
    (`KismetSystemLibrary.Delay` (`KismetMathLibrary.RandomFloatInRange` 1.0 2.0))
    (`self.StartFlickering`)))

(event `StartFlickering`
  ;[0 0 0] Flickering
  (bind (_direction _track) (`Timeline|LightFlickering` :!via `PlayFromStart` :!label _label)
    (:`Update`
      (`LightComponent.SetIntensity` (`self.PointLight`) (`KismetMathLibrary.Lerp` 1500.0 10000.0 _track)))
    (:`Finished`
      (`self.Reverse`))))

(event `Reverse`
  ;[0 0 0] Flickering
  (`/Engine/EditorBlueprintResources/StandardMacros.FlipFlop`
    (:`A`
      (goto _label :!via `Reverse`))
    (:`B`
      (goto _label :!via `PlayFromStart`))))

(fn `UserConstructionScript`
  (`LightComponent.SetIntensity` (`self.PointLight`) (`self.New Light Intensity`)))
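; BP_DecorationCore is a base sprite decoration prop that can optionally billboard toward the player and be destroyed by damage.
; Tick yaws its Direction component at the player when FaceToCamera is set.
; With AllowDamage on, damage goes through ACHealth; on destruction it spawns a zero-damage explosion, particles and sound, swaps to a destroyed sprite and disables collision.
; FDropItem then spawns an optional pickup class slightly above the prop.
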(event `self.ReceiveTick`
  (params (DeltaSeconds :type "Float (single-precision)"))
  (bind (_returnvalue_roll _returnvalue_pitch _returnvalue_yaw) (`KismetMathLibrary.BreakRotator` (`KismetMathLibrary.FindLookAtRotation` (`self.K2_GetActorLocation`) (`self.K2_GetActorLocation` (`GameplayStatics.GetPlayerCharacter` 0)))))
  ;[0 0 0] Tick Event
  (if (`self.FaceToCamera`)
    (`SceneComponent.K2_SetWorldRotation` (`self.Direction`) (`KismetMathLibrary.MakeRotator` 0.0 0.0 _returnvalue_yaw) false false)))

(event `self.ReceiveAnyDamage`
  (params (Damage :type "Float (single-precision)") (DamageType :type "DamageType Object Reference") (InstigatedBy :type "Controller Object Reference") (DamageCauser :type "Actor Object Reference"))
  (bind _returnvalue (`self.K2_GetActorLocation`))
  (bind _returnvalue_2 (`SceneComponent.K2_GetComponentLocation` (`self.Collision`)))
  ;[0 0 0] Any Damage
  (if (`self.AllowDamage?`)
    (if (not (`self.isDestroy?`))
      (bind _dead (`/Game/RetroBoomerFPSFramework/Blueprints/ActorComponents/AC_Health.ApplyDamage` (`self.AC_Health`) Damage))
      (bind _output_get (set `self.isDestroy?` _dead))
      (if _output_get
        (`|SpawnActorFromClass` "/Game/RetroBoomerFPSFramework/Blueprints/Interactables/BP_Explosion.BP_Explosion_C" (`KismetMathLibrary.MakeTransform` _returnvalue_2) "Undefined" "OverrideRootScale" null "/Game/RetroBoomerFPSFramework/Flipbooks/Props/FB_Explosion.FB_Explosion" 0.0 0.0 _returnvalue_2 0.0 0.0 0.0 0.5 null null null)
        (`GameplayStatics.SpawnEmitterAtLocation` null _returnvalue)
        (`GameplayStatics.PlaySoundAtLocation` (`self.ExplosionSound`) _returnvalue (struct) 1.0 1.0 0.0 null null null null)
        (`PaperSpriteComponent.SetSprite` (`self.PaperSprite`) (`self.DestroyedSprite`))
        (`PrimitiveComponent.SetCollisionEnabled` (`self.Collision`) "NoCollision")
        (`self.F_DropItem`)))))

(fn `F_DropItem`
  (bind (_returnvalue_x _returnvalue_y _returnvalue_z) (`KismetMathLibrary.BreakVector` (`self.K2_GetActorLocation`)))
  (if (`KismetSystemLibrary.IsValidClass` (`self.DropItem`))
    (`|SpawnActorFromClass` (`self.DropItem`) (`KismetMathLibrary.MakeTransform` (`KismetMathLibrary.MakeVector` _returnvalue_x _returnvalue_y (+ _returnvalue_z 20.0))) "Undefined" "OverrideRootScale" null null)))

(fn `UserConstructionScript`)
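; Game instance for a retro FPS that manages difficulty, game flow and level progression saved in an SG_Game slot.
; New game shows a popup if a save exists, then deletes the slot and opens the default level.
; Level completion updates the level's record, keeping the larger time and secret count, and unlocks the next on first completion.
; Continue restores difficulty and opens the highest unlocked level, or MainMenu if already there.
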(fn `GetLevelName`
  (params (CurrentLevel :type String))
  (returns (LevelName :type String))
  ;[0 0 0] Searches the saved game’s level list for the current level name and returns it, confirming whether the level exists in the player’s progression data.
  (bind _returnvalue (`GameplayStatics.LoadGameFromSlot` (`self.SlotName`)))
  (bind _assg_game (cast `/Game/RetroBoomerFPSFramework/Blueprints/SaveGame/SG_Game` _returnvalue))
  (for _array_element (`/Game/RetroBoomerFPSFramework/Blueprints/SaveGame/SG_Game.LevelList` _assg_game)
    (bind ((`UE_LevelName_18_74BAF7474B4BC2A8FC4D2687C6E6E37D` _ue_levelname) (`LevelName_19_25BE789E47594CC3A2D734A6DAF445C4` _levelname)) (break `/Game/RetroBoomerFPSFramework/Blueprints/Structures/S_LevelProgression` _array_element))
    (if (== _ue_levelname (`local.CurrentLevel`))
      (break)))
  (return _levelname))

(fn `HasSaveGame`
  (returns (ReturnValue :type Boolean))
  ;[0 0 0] Checks if a save game exists in the specified slot and returns true or false.
  (bind _returnvalue (`GameplayStatics.DoesSaveGameExist` (`self.SlotName`)))
  (return _returnvalue))

(fn `NewGame`
  (params (SetDifficulty :type "/Game/RetroBoomerFPSFramework/Blueprints/Enums/E_GameDifficulty Enum" :default "NewEnumerator0"))
  ;[0 0 0] Handles new game start logic by setting difficulty, checking for an existing save, and either showing a confirmation popup or starting the game directly.
  (set `self.Difficulty` SetDifficulty)
  (bind _returnvalue (`self.HasSaveGame`))
  (if _returnvalue
    (bind _returnvalue_2 (`|CreateWidget` "/Game/RetroBoomerFPSFramework/Blueprints/Widgets/MainMenu/WB_Popup.WB_Popup_C"))
    (`UserWidget.AddToViewport` _returnvalue_2 0)
    (add `/Game/RetroBoomerFPSFramework/Blueprints/Widgets/MainMenu/WB_Popup.OnClickOK` _returnvalue_2 (`|CreateDelegate` :!event `StartGame`))
    (else
      (`self.StartGame`))))

(fn `OnContinue`
  (bind _returnvalue (`self.HasSaveGame`))
  (if _returnvalue
    (bind _returnvalue_2 (`GameplayStatics.LoadGameFromSlot` (`self.SlotName`)))
    (bind _assg_game (cast `/Game/RetroBoomerFPSFramework/Blueprints/SaveGame/SG_Game` _returnvalue_2))
    (set `self.Difficulty` (`/Game/RetroBoomerFPSFramework/Blueprints/SaveGame/SG_Game.GameDifficulty` _assg_game))
    (bind _returnvalue_3 (`GameplayStatics.GetCurrentLevelName` true))
    (bind ((`UE_LevelName_18_74BAF7474B4BC2A8FC4D2687C6E6E37D` _ue_levelname)) (break `/Game/RetroBoomerFPSFramework/Blueprints/Structures/S_LevelProgression` (`|GetArrayItem` (`/Game/RetroBoomerFPSFramework/Blueprints/SaveGame/SG_Game.LevelList` _assg_game) (`/Game/RetroBoomerFPSFramework/Blueprints/SaveGame/SG_Game.HighestUnlockedLevel` _assg_game))))
    (if (== _returnvalue_3 _ue_levelname)
      (`GameplayStatics.OpenLevel` "MainMenu")
      (else
        (`GameplayStatics.OpenLevel` _ue_levelname)))))

(fn `OnLevelCompleted`
  (params (CurrentLevel :type String) (Progression :type "Float (double-precision)") (BestTime :type "Float (double-precision)") (Secrets :type Integer) (TotalSecrets :type Integer))
  ;[0 0 0] Saves progress when a level is completed by checking if a save file exists, loading or creating one, and then updating data such as level, progression, best time, secrets, and total score.
  (bind _returnvalue (`GameplayStatics.DoesSaveGameExist` (`self.SlotName`)))
  (if _returnvalue
    (bind _returnvalue_2 (`GameplayStatics.LoadGameFromSlot` (`self.SlotName`)))
    (bind _assg_game (cast `/Game/RetroBoomerFPSFramework/Blueprints/SaveGame/SG_Game` _returnvalue_2))
    (set `self.SG_Game` _assg_game)
    (else
      (bind _returnvalue_3 (`GameplayStatics.CreateSaveGameObject` "/Game/RetroBoomerFPSFramework/Blueprints/SaveGame/SG_Game.SG_Game_C"))
      (set `self.SG_Game` _returnvalue_3)))
  (`self.SaveGame` (`local.CurrentLevel`) (`local.Progression`) (`local.BestTime`) (`local.Secrets`) (`local.TotalSecrets`)))

(fn `SaveGame`
  (params (CurrentLevel :type String) (Progression :type "Float (double-precision)") (BestTime :type "Float (double-precision)") (Secrets :type Integer) (TotalSecrets :type Integer))
  (locals (LevelIdx :type Integer :default 0) (LevelRef :type "/Game/RetroBoomerFPSFramework/Blueprints/Structures/S_LevelProgression Structure"))
  (bind _secrets (`local.Secrets`))
  (bind _sg_game (`self.SG_Game`))
  (bind _besttime (`local.BestTime`))
  (bind ((`BestTime_31_DDA2BD4B4E8839D906CE92AC74DF1D88` _besttime_2) (`Secret_36_F855800543BFF4687D22ADBA077D44FB` _secret)) (break `/Game/RetroBoomerFPSFramework/Blueprints/Structures/S_LevelProgression` (`local.LevelRef`)))
  (bind _levellist (`/Game/RetroBoomerFPSFramework/Blueprints/SaveGame/SG_Game.LevelList` (`self.SG_Game`)))
  (for _array_element (`/Game/RetroBoomerFPSFramework/Blueprints/SaveGame/SG_Game.LevelList` (`self.SG_Game`))
    (if (== (`.UE_LevelName_18_74BAF7474B4BC2A8FC4D2687C6E6E37D` (break `/Game/RetroBoomerFPSFramework/Blueprints/Structures/S_LevelProgression` _array_element)) (`local.CurrentLevel`))
      (break)))
  (bind _returnvalue (`KismetArrayLibrary.Array_Find` _levellist _array_element))
  (set `local.LevelIdx` _returnvalue)
  (bind _output_get (set `local.LevelRef` (`|GetArrayItem` _levellist _returnvalue)))
  (if (not (`.Completed_15_9204C78B429A0E865187EAA2EA3078D9` (break `/Game/RetroBoomerFPSFramework/Blueprints/Structures/S_LevelProgression` _output_get)))
    (set `/Game/RetroBoomerFPSFramework/Blueprints/SaveGame/SG_Game.HighestUnlockedLevel` (`KismetMathLibrary.Clamp` (+ (`/Game/RetroBoomerFPSFramework/Blueprints/SaveGame/SG_Game.HighestUnlockedLevel` _sg_game) 1) 0 (`KismetArrayLibrary.Array_LastIndex` (`/Game/RetroBoomerFPSFramework/Blueprints/SaveGame/SG_Game.LevelList` _sg_game))) (`self.SG_Game`)))
  (set `/Game/RetroBoomerFPSFramework/Blueprints/SaveGame/SG_Game.GameDifficulty` (`self.Difficulty`) (`self.SG_Game`))
  (bind _structout (setmembers `/Game/RetroBoomerFPSFramework/Blueprints/Structures/S_LevelProgression` :`StructRef` (`local.LevelRef`) :`Progression` (`local.Progression`) :`BestTime` (`KismetMathLibrary.SelectFloat` _besttime_2 _besttime (>= _besttime_2 _besttime)) :`Secret` (`KismetMathLibrary.SelectInt` _secrets _secret (>= _secrets _secret)) :`TotalSecrets` (`local.TotalSecrets`) :`Completed` true))
  (`KismetArrayLibrary.Array_Set` (`/Game/RetroBoomerFPSFramework/Blueprints/SaveGame/SG_Game.LevelList` (`self.SG_Game`)) (`local.LevelIdx`) _structout)
  (`GameplayStatics.SaveGameToSlot` (`self.SG_Game`) (`self.SlotName`)))

(fn `StartGame`
  (`GameplayStatics.DeleteGameInSlot` (`self.SlotName`))
  (`GameplayStatics.OpenLevel` (`self.DefaultLevel`)))
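; Health and armor component for the Retro Boomer FPS framework that tracks damage and death for its owner.
; ApplyDamage drains armor first, passes any overflow to health, and returns whether the hit leaves the owner dead.
; SetHealth and SetArmor add the given amount to the current value rather than replacing it, returning the result.
; All changes clamp between zero and the respective maximum.
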(fn `ApplyDamage`
  (params (`DamageAmount ` :type "Float (double-precision)"))
  (returns (Dead :type Boolean))
  (locals (Absorb :type "Float (double-precision)") (DamageLeft :type "Float (double-precision)"))
  ;[0 0 0] This function processes incoming damage by first checking if the character has Armor.
  (if (> (`self.Armor`) 0.0)
    (set `local.Absorb` (`KismetMathLibrary.FMin` (`local.DamageAmount `) (`self.Armor`)))
    (set `self.Armor` (`KismetMathLibrary.FClamp` (- (`self.Armor`) (`local.Absorb`)) 0.0 (`self.MaxArmor`)))
    (set `local.DamageLeft` (- (`local.DamageAmount `) (`local.Absorb`)))
    (if (> (`self.Armor`) 0.0)
      (return false)
      (else
        (bind _output_get (set `self.Health` (`KismetMathLibrary.FClamp` (- (`self.Health`) (`local.DamageLeft`)) 0.0 (`self.MaxHealth`))))
        (return (<= _output_get 0.0))))
    (elif (<= (`self.Health`) 0.0)
      (return true) ; is Dead
      (else
        (bind _output_get_2 (set `self.Health` (`KismetMathLibrary.FClamp` (- (`self.Health`) (`local.DamageAmount `)) 0.0 (`self.MaxHealth`))))
        (return (<= _output_get_2 0.0))))))

(fn `Set_Armor`
  (params (Armor :type "Float (double-precision)"))
  (returns (NewArmor :type "Float (double-precision)"))
  ;[0 0 0] This function updates the character’s Armor value.
  (bind _output_get (set `self.Armor` (`KismetMathLibrary.FClamp` (+ Armor (`self.Armor`)) 0.0 (`self.MaxArmor`))))
  (return _output_get))

(fn `Set_Health`
  (params (Health :type "Float (double-precision)"))
  (returns (NewHealth :type "Float (double-precision)"))
  ;[0 0 0] This function updates the character’s Health value.
  (bind _output_get (set `self.Health` (`KismetMathLibrary.FClamp` (+ Health (`self.Health`)) 0.0 (`self.MaxHealth`))))
  (return _output_get))
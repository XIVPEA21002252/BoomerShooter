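; Base enemy for a retro boomer shooter: a billboarded Paper2D flipbook character that patrols, chases and attacks the player.
; Patrols randomly or between two points until PawnSensing latches onto the player, then chases and fires melee sphere traces or projectiles.
; Each tick, dot products against the player direction pick four-way flipbooks for idle, walk, hurt or attack.
; Difficulty scales health and damage; death updates the player's kill count and drops an optional item.
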(event `self.ReceiveTick`
  (params (DeltaSeconds :type "Float (single-precision)"))
  ;[0 0 0] Event Tick
  (`parent.ReceiveTick` DeltaSeconds)
  (`self.Set Sprite Face Player`)
  (`self.Set Enemy Face Target`)
  (`self.GetEnemyDirection`)
  (`self.SetMovementState`)
  (`self.SetEnemyFlipbook`)
  (`self.WalkAudio`))

(event `self.ReceiveBeginPlay`
  ;[0 0 0] Beginplay
  (`KismetSystemLibrary.Delay` 0.2)
  (`self.Setup`)
  (`self.PatrolState`)
  (`self.GetDifficultyParams`))

(event `DoMeleeAttack`
  (params (DamagedActor :type "/Game/RetroBoomerFPSFramework/Blueprints/Characters/BP_DefaultCharacter Object Reference"))
  (bind _shotmuzzle (`self.ShotMuzzle`))
  (bind _returnvalue (`SceneComponent.K2_GetComponentLocation` _shotmuzzle))
  ;[0 0 0] Enemy Attack
  ;;[0.1095 0.1095 0.1095] Melee Attack
  (if (`self.bSeeingPawn?`)
    (`/Engine/EditorBlueprintResources/StandardMacros.DoOnce` false :!label _label
      (:`Completed`
        (if (not (`/Game/RetroBoomerFPSFramework/Blueprints/Characters/BP_CharacterCore.isDead?` DamagedActor))
          (set `self.bAttack?` true)
          (`GameplayStatics.PlaySoundAtLocation` (`self.AttackSound`) (`self.K2_GetActorLocation`) (struct) 1.0 1.0 0.0 null null null null) ; Enemy Attack Sound Here
          (`KismetSystemLibrary.Delay` (`self.AttackAnimDuration`))
          (set `self.bAttack?` false)
          (`self.HasEnemyDie?`
            (:`false`
              (bind _outhit (`KismetSystemLibrary.SphereTraceSingleForObjects` _returnvalue (+ _returnvalue (* (`KismetMathLibrary.GetForwardVector` (`SceneComponent.K2_GetComponentRotation` _shotmuzzle)) (`self.AttackRange`))) 80.0 (`|MakeArray` "ObjectTypeQuery3" :!type "EObjectTypeQuery Enum") false (`|MakeArray` self :!type "Actor Object Reference") "None" false))
              (bind _asbp_default_character (cast `/Game/RetroBoomerFPSFramework/Blueprints/Characters/BP_DefaultCharacter` (`.HitActor` (`GameplayStatics.BreakHitResult` _outhit)))
                (:`then`
                  (`GameplayStatics.ApplyDamage` _asbp_default_character (`self.Damage`) null self (`self.DamageType`))
                  (`KismetSystemLibrary.Delay` (`self.DelayBetweenAttack`))
                  (goto _label :!via `Reset`))
                (:`CastFailed`
                  (goto _label :!via `Reset`))))))))))

(event `self.ReceiveAnyDamage`
  (params (Damage :type "Float (single-precision)") (DamageType :type "DamageType Object Reference") (InstigatedBy :type "Controller Object Reference") (DamageCauser :type "Actor Object Reference"))
  ;[0 0 0] Enemy Damage & Death
  ;;[0.1095 0.1095 0.1095] Any Damage
  (`self.HasEnemyDie?`
    (:`false`
      (bind _dead (`/Game/RetroBoomerFPSFramework/Blueprints/ActorComponents/AC_Health.ApplyDamage` (`self.AC_Health`) Damage))
      (bind _output_get (set `self.isDead?` _dead))
      (if _output_get
        (set `self.bHurt?` false)
        (`self.DoDeath`)
        (`/Engine/EditorBlueprintResources/StandardMacros.IncrementInt` (`/Game/RetroBoomerFPSFramework/Blueprints/Characters/BP_DefaultCharacter.EnemiesDefeated` (`self.PlayerCast`)))
        (else
          (`|ExecutionSequence`
            (:`then_0`
              (`/Engine/EditorBlueprintResources/StandardMacros.DoOnce` false :!label _label_2
                (:`Completed`
                  (set `self.bHurt?` true)
                  (`KismetSystemLibrary.Delay` 0.2)
                  (set `self.bHurt?` false)
                  (`KismetSystemLibrary.Delay` 0.5)
                  (goto _label_2 :!via `Reset`))))
            (:`then_1`
              ;;;[0.4844 0.4844 0.4844] Chase player if enemy gets hurt
              (`self.HasSeenPlayer?`
                (:`false`
                  (`|AIMoveTo` self (0.0 0.0 0.0) (`GameplayStatics.GetPlayerPawn` 0) (`self.TargetReachRadius`)))))))))))

(event `DoRangeAttack`
  ;[0 0 0] Enemy Attack
  ;;[0.1095 0.1095 0.1095] Range Attack
  (if (`self.bSeeingPawn?`)
    (`/Engine/EditorBlueprintResources/StandardMacros.DoOnce` false :!label _label_3
      (:`Completed`
        (set `self.bAttack?` true)
        (`GameplayStatics.PlaySoundAtLocation` (`self.AttackSound`) (`self.K2_GetActorLocation`) (struct) 1.0 1.0 0.0 null null null null) ; Enemy Attack Sound Here
        (`KismetSystemLibrary.Delay` (`self.AttackAnimDuration`))
        (set `self.bAttack?` false)
        (`self.HasEnemyDie?`
          (:`false`
            (`|SpawnActorFromClass` "/Game/RetroBoomerFPSFramework/Blueprints/Projectiles/BP_EnemyProjectile.BP_EnemyProjectile_C" (`SceneComponent.K2_GetComponentToWorld` (`self.ShotMuzzle`)) "AlwaysSpawn" "OverrideRootScale" null (`self.Damage`) (`self.Projectile Flipbook`) (`self.DamageType`) null)
            (`KismetSystemLibrary.Delay` (`self.DelayBetweenAttack`))
            (goto _label_3 :!via `Reset`)))))))

(event `self.DoDeath`
  ;[0 0 0] Enemy Damage & Death
  ;;[0.1095 0.1095 0.1095] Death Event
  (`GameplayStatics.PlaySoundAtLocation` (`self.DeathSound`) (`self.K2_GetActorLocation`) (struct) 1.0 1.0 0.0 null null null null) ; Enemy Death Sound Here
  (`CharacterMovementComponent.DisableMovement` (`self.CharacterMovement`))
  (`PrimitiveComponent.SetCollisionEnabled` (`self.CapsuleComponent`) "NoCollision")
  (`PaperFlipbookComponent.SetFlipbook` (`self.Sprite`) (`self.DeathAnimSprite`))
  (`KismetSystemLibrary.Delay` (`self.DeathEndAnimDelay`))
  (`PaperFlipbookComponent.SetFlipbook` (`self.Sprite`) (`self.StaticDeathSprite`))
  (`self.DropItemAfterDeath`)
  (if (`self.bCanDestroyEnemy?`)
    (`KismetSystemLibrary.Delay` (`self.DestroyDelay`))
    (`self.K2_DestroyActor`)))

(event `DropItemAfterDeath`
  (bind (_returnvalue_x _returnvalue_y _returnvalue_z) (`KismetMathLibrary.BreakVector` (`self.K2_GetActorLocation`)))
  ;[0 0 0] Enemy Damage & Death
  ;;[0.1095 0.1095 0.1095] Drop Item after enemy dies
  (`KismetSystemLibrary.Delay` 1.0)
  (bind _dropitem (`self.DropItem`)
    (:`then`
      (`|SpawnActorFromClass` _dropitem (`KismetMathLibrary.MakeTransform` (`KismetMathLibrary.MakeVector` _returnvalue_x (- _returnvalue_y 5.0) (- _returnvalue_z 100.0))) "Undefined" "OverrideRootScale" null null))
    (:`else`)))

(event `self.PawnSensing.OnSeePawn`
  (params (Pawn :type "Pawn Object Reference"))
  ;[0 0 0] AI Behavior
  ;;[0.1714 0.1714 0.1714] On Pawn Sensing
  (`self.HasEnemyDie?`
    (:`false`
      (bind _asbp_default_character (cast `/Game/RetroBoomerFPSFramework/Blueprints/Characters/BP_DefaultCharacter` Pawn))
      (if (not (`/Game/RetroBoomerFPSFramework/Blueprints/Characters/BP_CharacterCore.isDead?` _asbp_default_character))
        (set `self.bSeeingPawn?` true)
        (set `CharacterMovementComponent.MaxWalkSpeed` (`self.ChaseMovementSpeed`) (`self.CharacterMovement`))
        (`|AIMoveTo` self (0.0 0.0 0.0) _asbp_default_character (`self.TargetReachRadius`)
          (:`OnSuccess`
            (`self.AttackType`)))))))

(event `BetweenTwoPoints`
  ;[0 0 0] AI Behavior
  ;;[0.1714 0.1714 0.1714] Between Two Points
  (`self.HasSeenPlayer?` :!label _label_4
    (:`false`
      (`|AIMoveTo` self (0.0 0.0 0.0) (`self.TargetLocation1`)
        (:`OnSuccess`
          _)
        (:`OnFail`
          _))
      (`self.HasSeenPlayer?`
        (:`false`
          (`KismetSystemLibrary.Delay` 3.0)
          (`self.HasSeenPlayer?`
            (:`false`
              (`|AIMoveTo` self (0.0 0.0 0.0) (`self.TargetLocation2`)
                (:`OnSuccess`
                  _)
                (:`OnFail`
                  _))
              (`self.HasSeenPlayer?`
                (:`false`
                  (`KismetSystemLibrary.Delay` 3.0)
                  (`self.HasSeenPlayer?`
                    (:`false`
                      (goto _label_4))))))))))))

(event `RandomPatrol`
  ;[0 0 0] AI Behavior
  ;;[0.1714 0.1714 0.1714] Random Patrol
  (bind _randomlocation (`NavigationSystemV1.K2_GetRandomLocationInNavigableRadius` (`self.K2_GetActorLocation`) 250.0 null null :!label _label_5))
  (`self.HasEnemyDie?`
    (:`false`
      (`self.HasSeenPlayer?`
        (:`false`
          (`|AIMoveTo` self _randomlocation null
            (:`OnSuccess`
              _)
            (:`OnFail`
              _))
          (`self.HasSeenPlayer?`
            (:`false`
              (`KismetSystemLibrary.Delay` 4.0)
              (`self.HasSeenPlayer?`
                (:`false`
                  (goto _label_5))))))))))

(fn `AttackType`
  ;[0 0 0] Executes the enemy’s attack logic, checking if alive and choosing between melee or ranged attack based on the attack type.
  (`self.HasEnemyDie?`
    (:`false`
      (if (`self.isMeleeEnemy?`)
        (`self.DoMeleeAttack` (`self.PlayerCast`))
        (else
          (`self.DoRangeAttack`))))))

(fn `GetActorData`
  (returns (`isInteractable?` :type Boolean) (TextTitle :type Text) (CurHealth :type "Float (double-precision)") (MaxHealth :type "Float (double-precision)"))
  (bind _ac_health (`self.AC_Health`))
  (return false (`self.EnemyName`) (`/Game/RetroBoomerFPSFramework/Blueprints/ActorComponents/AC_Health.Health` _ac_health) (`/Game/RetroBoomerFPSFramework/Blueprints/ActorComponents/AC_Health.MaxHealth` _ac_health)))

(fn `GetDifficultyParams`
  (locals (Difficulty :type "/Game/RetroBoomerFPSFramework/Blueprints/Enums/E_GameDifficulty Enum" :default "NewEnumerator0"))
  (bind _ac_health (`self.AC_Health`))
  (bind _health (`/Game/RetroBoomerFPSFramework/Blueprints/ActorComponents/AC_Health.Health` (`self.AC_Health`)))
  ;[0 0 0] Retrieves difficulty parameters from the Game Instance and adjusts enemy health and damage values according to the selected difficulty level.
  (bind _asgi_main (cast `/Game/RetroBoomerFPSFramework/Blueprints/GameInstance/GI_Main` (`GameplayStatics.GetGameInstance`)))
  (set `local.Difficulty` (`/Game/RetroBoomerFPSFramework/Blueprints/GameInstance/GI_Main.Difficulty` _asgi_main))
  (bind _output_get (set `/Game/RetroBoomerFPSFramework/Blueprints/ActorComponents/AC_Health.Health` (select `/Game/RetroBoomerFPSFramework/Blueprints/Enums/E_GameDifficulty` (`local.Difficulty`) :`NewEnumerator0` _health :`NewEnumerator1` (+ _health 50.0) :`NewEnumerator2` (+ _health 150.0)) _ac_health))
  (set `/Game/RetroBoomerFPSFramework/Blueprints/ActorComponents/AC_Health.MaxHealth` _output_get _ac_health)
  (set `self.Damage` (select `/Game/RetroBoomerFPSFramework/Blueprints/Enums/E_GameDifficulty` (`local.Difficulty`) :`NewEnumerator0` (`self.Damage`) :`NewEnumerator1` (+ (`self.Damage`) 5.0) :`NewEnumerator2` (+ (`self.Damage`) 15.0) :!type "Float (single-precision)")))

(fn `GetEnemyDirection`
  (locals (FacingRight :type Boolean))
  (bind (_returnvalue_x _returnvalue_y) (`KismetMathLibrary.BreakVector` (`self.GetActorForwardVector`)))
  (bind (_returnvalue_x_2 _returnvalue_y_2) (`KismetMathLibrary.BreakVector` (`self.GetActorRightVector`)))
  (bind (_returnvalue_x_3 _returnvalue_y_3) (`KismetMathLibrary.BreakVector` (`self.K2_GetActorLocation`)))
  (bind (_returnvalue_x_4 _returnvalue_y_4) (`KismetMathLibrary.BreakVector` (`self.K2_GetActorLocation` (`GameplayStatics.GetPlayerCharacter` 0))))
  (bind _returnvalue (`KismetMathLibrary.Normal` (- (`KismetMathLibrary.MakeVector` _returnvalue_x_4 _returnvalue_y_4) (`KismetMathLibrary.MakeVector` _returnvalue_x_3 _returnvalue_y_3))))
  (set `self.SpriteAngle` (`KismetMathLibrary.DegAcos` (`KismetMathLibrary.Dot_VectorVector` (`KismetMathLibrary.MakeVector` _returnvalue_x _returnvalue_y) _returnvalue)))
  (set `local.FacingRight` (> (`KismetMathLibrary.Dot_VectorVector` _returnvalue (`KismetMathLibrary.MakeVector` _returnvalue_x_2 _returnvalue_y_2)) 0.0))
  (if (< (`self.SpriteAngle`) 20.0)
    (set `self.MovementDirection` "NewEnumerator0")
    (return)
    (elif (< (`self.SpriteAngle`) 65.0)
      (set `self.MovementDirection` (select `bool` (`local.FacingRight`) :`false` "NewEnumerator2" :`true` "NewEnumerator3" :!type "/Game/RetroBoomerFPSFramework/Blueprints/Enums/E_MovementDirection Enum"))
      (return)
      (elif (< (`self.SpriteAngle`) 115.0)
        (set `self.MovementDirection` (select `bool` (`local.FacingRight`) :`false` "NewEnumerator2" :`true` "NewEnumerator3" :!type "/Game/RetroBoomerFPSFramework/Blueprints/Enums/E_MovementDirection Enum"))
        (return)
        (elif (< (`self.SpriteAngle`) 160.0)
          (set `self.MovementDirection` (select `bool` (`local.FacingRight`) :`false` "NewEnumerator2" :`true` "NewEnumerator3" :!type "/Game/RetroBoomerFPSFramework/Blueprints/Enums/E_MovementDirection Enum"))
          (return)
          (else
            (set `self.MovementDirection` "NewEnumerator1")
            (return)))))))

(fn `PatrolState`
  ;[0 0 0] Sets the enemy’s patrol behavior by adjusting walk speed and selecting between idle, random patrol, or moving between two points based on AI patrol mode
  (set `CharacterMovementComponent.MaxWalkSpeed` (`self.WalkMovementSpeed`) (`self.CharacterMovement`))
  (switch `/Game/RetroBoomerFPSFramework/Blueprints/Enums/E_AI_PatrolMode` (`self.AIPatrolMode`)
    (:`NewEnumerator1`
      (`self.RandomPatrol`))
    (:`NewEnumerator2`
      (`self.BetweenTwoPoints`))))

(fn `Set Enemy Face Target`
  (bind (_returnvalue_roll _returnvalue_pitch _returnvalue_yaw) (`KismetMathLibrary.BreakRotator` (`KismetMathLibrary.FindLookAtRotation` (`SceneComponent.K2_GetComponentLocation` (`self.CapsuleComponent`)) (`self.K2_GetActorLocation` (`GameplayStatics.GetPlayerCharacter` 0)))))
  ;[0 0 0] Rotates the enemy capsule to face the player when the AI has detected them.
  (`self.HasSeenPlayer?`
    (:`true`
      (`SceneComponent.K2_SetWorldRotation` (`self.CapsuleComponent`) (`KismetMathLibrary.MakeRotator` 0.0 0.0 _returnvalue_yaw) false false))))

(fn `Set Sprite Face Player`
  (bind (_returnvalue_roll _returnvalue_pitch _returnvalue_yaw) (`KismetMathLibrary.BreakRotator` (`KismetMathLibrary.FindLookAtRotation` (`SceneComponent.K2_GetComponentLocation` (`self.Sprite`)) (`self.K2_GetActorLocation` (`GameplayStatics.GetPlayerCharacter` 0)))))
  ;[0 0 0] Rotates the enemy sprite to always face the player using a look-at rotation with a yaw offset
  (`SceneComponent.K2_SetWorldRotation` (`self.Sprite`) (`KismetMathLibrary.MakeRotator` 0.0 0.0 (- _returnvalue_yaw 90.0)) false false))

(fn `SetEnemyFlipbook`
  ;[0 0 0] Set enemy Flipbook
  (`self.HasEnemyDie?`
    (:`false`
      (switch `/Game/RetroBoomerFPSFramework/Blueprints/Enums/E_MovementDirection` (`self.MovementDirection`)
        (:`NewEnumerator0`
          (`PaperFlipbookComponent.SetFlipbook` (`self.Sprite`) (select `/Game/RetroBoomerFPSFramework/Blueprints/Enums/E_CharacterState` (`self.CharacterState`) :`NewEnumerator0` (`|GetArrayItem` (`self.IdleSprites`)) :`NewEnumerator1` (`|GetArrayItem` (`self.WalkSprites`)) :`NewEnumerator3` (`|GetArrayItem` (`self.HurtSprites`)) :`NewEnumerator2` (`|GetArrayItem` (`self.AttackSprites`)))))
        (:`NewEnumerator1`
          (`PaperFlipbookComponent.SetFlipbook` (`self.Sprite`) (select `/Game/RetroBoomerFPSFramework/Blueprints/Enums/E_CharacterState` (`self.CharacterState`) :`NewEnumerator0` (`|GetArrayItem` (`self.IdleSprites`) 1) :`NewEnumerator1` (`|GetArrayItem` (`self.WalkSprites`) 1) :`NewEnumerator3` (`|GetArrayItem` (`self.HurtSprites`) 1) :`NewEnumerator2` (`|GetArrayItem` (`self.AttackSprites`) 1))))
        (:`NewEnumerator2`
          (`PaperFlipbookComponent.SetFlipbook` (`self.Sprite`) (select `/Game/RetroBoomerFPSFramework/Blueprints/Enums/E_CharacterState` (`self.CharacterState`) :`NewEnumerator0` (`|GetArrayItem` (`self.IdleSprites`) 2) :`NewEnumerator1` (`|GetArrayItem` (`self.WalkSprites`) 2) :`NewEnumerator3` (`|GetArrayItem` (`self.HurtSprites`) 2) :`NewEnumerator2` (`|GetArrayItem` (`self.AttackSprites`) 2))))
        (:`NewEnumerator3`
          (`PaperFlipbookComponent.SetFlipbook` (`self.Sprite`) (select `/Game/RetroBoomerFPSFramework/Blueprints/Enums/E_CharacterState` (`self.CharacterState`) :`NewEnumerator0` (`|GetArrayItem` (`self.IdleSprites`) 3) :`NewEnumerator1` (`|GetArrayItem` (`self.WalkSprites`) 3) :`NewEnumerator3` (`|GetArrayItem` (`self.HurtSprites`) 3) :`NewEnumerator2` (`|GetArrayItem` (`self.AttackSprites`) 3))))))))

(fn `SetMovementState`
  ;[0 0 0] Determine what state the enemy should be in
  (`self.HasEnemyDie?`
    (:`false`
      (if (`self.bAttack?`)
        (set `self.CharacterState` "NewEnumerator2")
        (elif (`self.bHurt?`)
          (set `self.CharacterState` "NewEnumerator3")
          (elif (> (`KismetMathLibrary.VSize` (`MovementComponent.Velocity` (`self.CharacterMovement`))) 1.0)
            (set `self.CharacterState` "NewEnumerator1")
            (else
              (set `self.CharacterState` "NewEnumerator0"))))))))

(fn `Setup`
  ;[0 0 0] Casts to the player character, sets the player reference, and increments the total Enemies to Defeat count for later display in the results widget.
  (bind _asbp_default_character (cast `/Game/RetroBoomerFPSFramework/Blueprints/Characters/BP_DefaultCharacter` (`GameplayStatics.GetPlayerCharacter` 0)))
  (bind _output_get (set `self.PlayerCast` _asbp_default_character))
  (`/Engine/EditorBlueprintResources/StandardMacros.IncrementInt` (`/Game/RetroBoomerFPSFramework/Blueprints/Characters/BP_DefaultCharacter.EnemiesToDefeat` _output_get)))

(fn `UserConstructionScript`
  (bind _ac_health (`self.AC_Health`))
  (`parent.UserConstructionScript`)
  (`AudioComponent.SetSound` (`self.AC_MoveLoop`) (`self.MoveWalkSound`))
  (bind _output_get (set `/Game/RetroBoomerFPSFramework/Blueprints/ActorComponents/AC_Health.Health` (`self.Health`) _ac_health))
  (set `/Game/RetroBoomerFPSFramework/Blueprints/ActorComponents/AC_Health.MaxHealth` _output_get _ac_health))

(fn `WalkAudio`
  (locals (Speed :type "Float (double-precision)" :default 0.0))
  ;[0 0 0] Plays and controls the walking loop audio by activating it when the player’s movement speed is above a set threshold.
  (bind _output_get (set `local.Speed` (`KismetMathLibrary.VSize` (`self.GetVelocity`))))
  (`ActorComponent.SetActive` (`self.AC_MoveLoop`) (> _output_get 100.0) false))
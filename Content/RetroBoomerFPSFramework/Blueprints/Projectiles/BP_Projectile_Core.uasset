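; BP_Projectile_Core is a projectile, apparently the framework's base, that handles impact damage and effects.
; On hit, it applies damage with the DAT_Lava damage type, spawns a particle effect and places a short-lived, randomly sized decal aligned to the surface normal.
; A dynamic material instance randomizes the decal's FrameIndex for visual variety.
; ApplyPhysics pushes simulating components with a velocity-scaled impulse, then the projectile destroys itself.
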(event `self.ReceiveHit`
  (params (MyComp :type "PrimitiveComponent Object Reference") (Other :type "Actor Object Reference") (OtherComp :type "PrimitiveComponent Object Reference") (bSelfMoved :type Boolean) (HitLocation :type "Vector Structure") (HitNormal :type "Vector Structure") (NormalImpulse :type "Vector Structure") (Hit :type "HitResult Structure (by ref)"))
  (bind (_bblockinghit _binitialoverlap _time _distance _location _impactpoint _normal _impactnormal _physmat _hitactor) (`GameplayStatics.BreakHitResult` Hit))
  (`GameplayStatics.ApplyDamage` _hitactor (`self.ProjectileDamage`) (`self.GetInstigatorController` (`self.GetInstigator`)) self "/Game/RetroBoomerFPSFramework/Blueprints/DamageType/DAT_Lava.DAT_Lava_C")
  (`GameplayStatics.SpawnEmitterAtLocation` (`self.ParticleFX`) _location)
  (bind _returnvalue (`GameplayStatics.SpawnDecalAtLocation` (`self.DecalMaterial`) (`KismetMathLibrary.Conv_IntToVector` (`KismetMathLibrary.RandomIntegerInRange` 8 15)) _location (`KismetMathLibrary.MakeRotFromX` _normal) 5.0))
  (bind _returnvalue_2 (`DecalComponent.CreateDynamicMaterialInstance` _returnvalue))
  (`MaterialInstanceDynamic.SetScalarParameterValue` _returnvalue_2 "FrameIndex" (`KismetMathLibrary.RandomFloatInRange` 0.0 8.0))
  (`self.ApplyPhysics` MyComp)
  (`/Engine/EditorBlueprintResources/StandardMacros.IsValid` self
    (:`Is Valid`
      (`self.K2_DestroyActor`))))

(fn `ApplyPhysics`
  (params (OtherComponent :type "PrimitiveComponent Object Reference"))
  (`/Engine/EditorBlueprintResources/StandardMacros.IsValid` (`local.OtherComponent`)
    (:`Is Valid`
      (if (`SceneComponent.IsSimulatingPhysics` (`local.OtherComponent`) "None")
        (`PrimitiveComponent.AddImpulseAtLocation` (`local.OtherComponent`) (* (`self.GetVelocity`) (`self.ProjectileImpulseStrenght`)) (`self.K2_GetActorLocation`) "None")
        (return)
        (else
          (return))))
    (:`Is Not Valid`
      (return))))

(fn `UserConstructionScript`)
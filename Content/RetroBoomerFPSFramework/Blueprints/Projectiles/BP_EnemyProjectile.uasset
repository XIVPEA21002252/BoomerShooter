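; Enemy projectile for a retro FPS that deals point damage on impact, shown as a flipbook sprite.
; The construction script applies the configured flipbook, and each tick yaws the sprite toward the player character as a yaw-only billboard.
; On hit it applies damage unless the hit actor matches the BP_Enemy_Core check, then destroys itself either way.
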(event `self.ReceiveTick`
  (params (DeltaSeconds :type "Float (single-precision)"))
  (`self.Set Sprite Face Player`))

(event `self.ReceiveHit`
  (params (MyComp :type "PrimitiveComponent Object Reference") (Other :type "Actor Object Reference") (OtherComp :type "PrimitiveComponent Object Reference") (bSelfMoved :type Boolean) (HitLocation :type "Vector Structure") (HitNormal :type "Vector Structure") (NormalImpulse :type "Vector Structure") (Hit :type "HitResult Structure (by ref)"))
  (if (!= Hit_HitActor "/Game/RetroBoomerFPSFramework/Blueprints/Enemies/BP_Enemy_Core.BP_Enemy_Core")
    (`GameplayStatics.ApplyPointDamage` Hit_HitActor (`self.Base Damage`) HitLocation (`GameplayStatics.MakeHitResult` Hit_bBlockingHit Hit_bInitialOverlap Hit_Time 0.0 Hit_Location Hit_ImpactPoint Hit_Normal Hit_ImpactNormal Hit_PhysMat Hit_HitActor Hit_HitComponent Hit_HitBoneName "None" Hit_HitItem 0 Hit_FaceIndex Hit_TraceStart Hit_TraceEnd) null null (`self.Damage Type Class`)))
  (`self.K2_DestroyActor`))

(fn `Set Sprite Face Player`
  (bind (_returnvalue_roll _returnvalue_pitch _returnvalue_yaw) (`KismetMathLibrary.BreakRotator` (`KismetMathLibrary.FindLookAtRotation` (`SceneComponent.K2_GetComponentLocation` (`self.FP_Fireball`)) (`self.K2_GetActorLocation` (`GameplayStatics.GetPlayerCharacter` 0)))))
  (`SceneComponent.K2_SetWorldRotation` (`self.FP_Fireball`) (`KismetMathLibrary.MakeRotator` 0.0 0.0 (- _returnvalue_yaw 90.0)) false false))

(fn `UserConstructionScript`
  (`PaperFlipbookComponent.SetFlipbook` (`self.FP_Fireball`) (`self.ProjectileFlipbook`)))
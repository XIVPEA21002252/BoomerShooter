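; Base weapon actor for a retro FPS, serving as both a player-facing sprite pickup and the equipped gun.
; Pickup adds it to the character's inventory and switches to it, or refills an owned copy's reserve ammo.
; Firing spawns spread projectiles with sound and a light flash, using a looping timer for automatic fire and delayed magazine reloads.
; Tick derives an idle, shoot or reload state from flags to choose the weapon flipbook.
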(event `self.ReceiveTick`
  (params (DeltaSeconds :type "Float (single-precision)"))
  ;[0 0 0 1 22] Event Tick
  (`self.FacePickupItem`)
  (`self.SetWeaponState`)
  (`self.SetWeaponFlipbook`))

(event `self.ReceiveBeginPlay`
  ;[0 0 0 1 22] Event beginplay
  (`parent.ReceiveBeginPlay`)
  (`self.Setup`))

(event `OnFire`
  ;[0 0 0 1 22] Fire Event called from character
  (`/Engine/EditorBlueprintResources/StandardMacros.DoOnce` false :!label _label
    (:`Completed`
      (`|ExecutionSequence`
        (:`then_0`
          (if (`self.isReloading?`)
            _
            (elif (`self.isAutomatic`)
              (`self.StartWeaponFire`)
              (`KismetSystemLibrary.K2_SetTimerDelegate` (delegate `StartWeaponFire`) (`self.AutomaticFire Rate`) true)
              (elif (`self.Infinite Ammo`)
                (if (not (and (not (`self.isReloading?`)) (`/Game/RetroBoomerFPSFramework/Blueprints/Characters/BP_CharacterCore.isDead?` (`self.PlayerCast`)))) :!label _label_2
                  (set `self.isShooting?` true)
                  (`GameplayStatics.SpawnSoundAtLocation` (`self.Fire Sound`) (`self.K2_GetActorLocation`) (struct) 1.0 1.0 0.0 null null) ; Firing Sound
                  (`|ExecutionSequence`
                    (:`then_0`
                      (`self.DoShoot`)
                      (`KismetSystemLibrary.RetriggerableDelay` (`self.ShotAnimDuration`))
                      (set `self.isShooting?` false)
                      (if (not (> (`self.CurrentMagAmmo`) 0))
                        (`self.ReloadWeapon`)))
                    (:`then_1`
                      ;;[0.1562 0.1562 0.1562] Anim Fire Light
                      (bind (_direction _value) (`Timeline|LightSource` :!via `PlayFromStart`)
                        (:`Update`
                          (`LightComponent.SetIntensity` (`self.FIreLight`) (`KismetMathLibrary.Lerp` 0.0 (`self.FireLightIntensity`) _value)))))))
                (else
                  (bind _canfire_ (`self.CheckAmmo` :!label _label_3))
                  (if _canfire_
                    (goto _label_2)
                    (else
                      (`self.ReloadWeapon`))))))))
        (:`then_1`
          (`KismetSystemLibrary.RetriggerableDelay` (`self.DelayBetweenShot`))
          (goto _label :!via `Reset`))))))

(event `StartWeaponFire`
  ;[0 0 0 1 22] Fire Event called from character
  (if (`self.Infinite Ammo`)
    (goto _label_2)
    (else
      (goto _label_3))))

(event `StopFire`
  ;[0 0 0 1 22] Fire Event called from character
  ;;[0 0 0] Stop Fire Event (Clear timer)
  (`KismetSystemLibrary.K2_ClearTimer` null "StartWeaponFire"))

(event `ReloadWeapon`
  ;[0 0 0 1 22] Reloading
  (if (`self.CanReload?`)
    (`KismetSystemLibrary.K2_ClearTimer` null "StartWeaponFire")
    (bind _canreload_ (`self.CheckAmmoMagazine`))
    (if _canreload_
      (if (not (and (`self.isReloading?`) (`self.isShooting?`)))
        (set `self.isReloading?` true)
        (`GameplayStatics.SpawnSoundAtLocation` (`self.Reload Sound`) (`self.K2_GetActorLocation`) (struct) 1.0 1.0 0.0 null null) ; Reload Sound
        (`KismetSystemLibrary.Delay` (`self.ReloadTime`))
        (`self.UpdateAmmo`)
        (set `self.isReloading?` false)
        (set `self.isShooting?` false)))))

(event `self.SpherePickup.OnComponentBeginOverlap`
  (params (OverlappedComponent :type "PrimitiveComponent Object Reference") (OtherActor :type "Actor Object Reference") (OtherComp :type "PrimitiveComponent Object Reference") (OtherBodyIndex :type Integer) (bFromSweep :type Boolean) (SweepResult :type "HitResult Structure (by ref)"))
  ;[0 0 0 1 22] Checks if the weapon being picked up is not already in the inventory. If not present, adds it to the inventory. If present, checks if its ammo is below the maximum. If below max, increases the ammo of the matching weapon in the inventory and destroys the pickup. If at or above max, does nothing and leaves the pickup in the world.
  ;;[0.162 0.162 0.162] Overlap Weapon
  (bind _asbp_default_character (cast `/Game/RetroBoomerFPSFramework/Blueprints/Characters/BP_DefaultCharacter` OtherActor))
  (`self.Interact` _asbp_default_character))

(event `Interact`
  (params (Playercast :type "/Game/RetroBoomerFPSFramework/Blueprints/Characters/BP_DefaultCharacter Object Reference"))
  ;[0 0 0 1 22] Checks if the weapon being picked up is not already in the inventory. If not present, adds it to the inventory. If present, checks if its ammo is below the maximum. If below max, increases the ammo of the matching weapon in the inventory and destroys the pickup. If at or above max, does nothing and leaves the pickup in the world.
  ;;[0.162 0.162 0.162] Interact with Weapon to Pickup
  (set `self.PlayerCast` Playercast)
  (if (not (`self.isTaken?`))
    (set `self.HasWeapon?` false)
    (for _array_element (`/Game/RetroBoomerFPSFramework/Blueprints/Characters/BP_DefaultCharacter.ArmoryInventory` (`self.PlayerCast`))
      (if (== (`GameplayStatics.GetObjectClass` _array_element) (`GameplayStatics.GetObjectClass` self))
        (set `self.HasWeapon?` true)
        (break)))
    (if (`self.HasWeapon?`)
      (if (< (`/Game/RetroBoomerFPSFramework/Blueprints/Weapon/Core/BP_Weapon_Core.CurrentClipAmmo` _array_element) (`/Game/RetroBoomerFPSFramework/Blueprints/Weapon/Core/BP_Weapon_Core.MaxClipAmmo` _array_element))
        (set `/Game/RetroBoomerFPSFramework/Blueprints/Weapon/Core/BP_Weapon_Core.CurrentClipAmmo` (`/Game/RetroBoomerFPSFramework/Blueprints/Weapon/Core/BP_Weapon_Core.MaxClipAmmo` _array_element) _array_element)
        (`/Game/RetroBoomerFPSFramework/Blueprints/Characters/BP_DefaultCharacter.SendNotification` (`self.PlayerCast`) (`|FormatText` "You got {name} Max Ammo" (`self.Weapon Name`)))
        (`GameplayStatics.PlaySound2D` "/Game/RetroBoomerFPSFramework/Sounds/SFX/General/Cue/Cue_GameArmorOn.Cue_GameArmorOn" 1.0 1.0 0.0 null null)
        (`self.K2_DestroyActor`))
      (else
        (`PrimitiveComponent.SetCollisionEnabled` (`self.SpherePickup`) "NoCollision")
        (set `self.isTaken?` true)
        (`self.AddNewWeapon`)
        (`/Game/RetroBoomerFPSFramework/Blueprints/Characters/BP_DefaultCharacter.SendNotification` (`self.PlayerCast`) (`|FormatText` "You got the {name}" (`self.Weapon Name`)))))))

(event `StarterWeapon`
  (params (Playercast :type "/Game/RetroBoomerFPSFramework/Blueprints/Characters/BP_DefaultCharacter Object Reference"))
  ;[0 0 0 1 22] Checks if the weapon being picked up is not already in the inventory. If not present, adds it to the inventory. If present, checks if its ammo is below the maximum. If below max, increases the ammo of the matching weapon in the inventory and destroys the pickup. If at or above max, does nothing and leaves the pickup in the world.
  ;;[0.162 0.162 0.162] Equip Starter Weapon
  (set `self.PlayerCast` Playercast)
  (if (not (`self.isTaken?`))
    (set `self.HasWeapon?` false)
    (`PrimitiveComponent.SetCollisionEnabled` (`self.SpherePickup`) "NoCollision")
    (set `self.isTaken?` true)
    (`self.AddNewWeapon`)))

(fn `AddNewWeapon`
  (bind _weaponidx (`/Game/RetroBoomerFPSFramework/Blueprints/Characters/BP_DefaultCharacter.AddWeapon` (`self.PlayerCast`) (`self.SpawnedWeapon`)))
  (`/Game/RetroBoomerFPSFramework/Blueprints/Characters/BP_DefaultCharacter.SwitchingWeapon` (`self.PlayerCast`) _weaponidx)
  (set `self.isTaken?` true)
  (`PrimitiveComponent.SetCollisionEnabled` (`self.SpherePickup`) "NoCollision")
  (`SceneComponent.SetVisibility` (`self.PickupSprite`) false false)
  (`SceneComponent.SetVisibility` (`self.WeaponSprite`) true false)
  (`TextRenderComponent.K2_SetText` (`self.TitleName`) (`KismetTextLibrary.Conv_StringToText` "")))

(fn `CheckAmmo`
  (returns (`CanFire?` :type Boolean))
  (if (> (`self.CurrentMagAmmo`) 0)
    (set `self.CurrentMagAmmo` (- (`self.CurrentMagAmmo`) 1))
    (return true)
    (else
      (return false))))

(fn `CheckAmmoMagazine`
  (returns (`CanReload?` :type Boolean))
  (return (and (< (`self.CurrentMagAmmo`) (`self.MaxMagAmmo`)) (>= (`self.CurrentClipAmmo`) 1))))

(fn `DoShoot`
  (bind _spreadx (`self.SpreadX`))
  (bind _playercast (`self.PlayerCast`))
  (bind _spready (`self.SpreadY`))
  (bind (_returnvalue_roll _returnvalue_pitch _returnvalue_yaw) (`KismetMathLibrary.BreakRotator` (`SceneComponent.K2_GetComponentRotation` (`self.BulletSpawn`))))
  (for _ (range (+ (`self.AdditionalProjectile`) 1))
    (`|SpawnActorFromClass` (`self.ProjectileType`) (`KismetMathLibrary.MakeTransform` (`SceneComponent.K2_GetComponentLocation` (`self.BulletSpawn`)) (`KismetMathLibrary.MakeRotator` _returnvalue_roll (+ _returnvalue_pitch (`KismetMathLibrary.RandomFloatInRange` (* _spready -1.0) _spready)) (+ _returnvalue_yaw (`KismetMathLibrary.RandomFloatInRange` (* _spreadx -1.0) _spreadx)))) "AlwaysSpawn" "OverrideRootScale" _playercast (`self.WeaponDamage`) _playercast)))

(fn `FacePickupItem`
  (bind (_returnvalue_roll _returnvalue_pitch _returnvalue_yaw) (`KismetMathLibrary.BreakRotator` (`KismetMathLibrary.FindLookAtRotation` (`self.K2_GetActorLocation`) (`self.K2_GetActorLocation` (`GameplayStatics.GetPlayerCharacter` 0)))))
  (if (not (`self.isTaken?`))
    (`SceneComponent.K2_SetWorldRotation` (`self.Arrow`) (`KismetMathLibrary.MakeRotator` 0.0 0.0 _returnvalue_yaw) false false)))

(fn `Setup`
  (bind _asbp_default_character (cast `/Game/RetroBoomerFPSFramework/Blueprints/Characters/BP_DefaultCharacter` (`GameplayStatics.GetPlayerCharacter` 0)))
  (set `self.PlayerCast` _asbp_default_character)
  (set `self.SpawnedWeapon` self)
  (`TextRenderComponent.K2_SetText` (`self.TitleName`) (`self.Weapon Name`))
  (`LightComponent.SetLightColor` (`self.FIreLight`) (`self.FireLightColor`) true)
  (set `self.CurrentMagAmmo` (`self.MaxMagAmmo`))
  (set `self.CurrentClipAmmo` (`self.MaxClipAmmo`)))

(fn `SetWeaponFlipbook`
  (switch `/Game/RetroBoomerFPSFramework/Blueprints/Enums/E_WeaponState` (`self.WeaponState`)
    (:`NewEnumerator0`
      (`PaperFlipbookComponent.SetFlipbook` (`self.WeaponSprite`) (`self.Idle Flipbook`)))
    (:`NewEnumerator1`
      (`PaperFlipbookComponent.SetFlipbook` (`self.WeaponSprite`) (`self.Shoot Flipbook`)))
    (:`NewEnumerator2`
      (`PaperFlipbookComponent.SetFlipbook` (`self.WeaponSprite`) (`self.ReloadFlipbook`)))))

(fn `SetWeaponState`
  ;[0 0 0] Determine what state the weapon should be in
  (if (`self.isReloading?`)
    (set `self.WeaponState` "NewEnumerator2")
    (elif (`self.isShooting?`)
      (set `self.WeaponState` "NewEnumerator1")
      (else
        (set `self.WeaponState` "NewEnumerator0")))))

(fn `UpdateAmmo`
  (locals (RequieredAmmo :type Integer))
  (bind _returnvalue (- (`self.CurrentClipAmmo`) (`local.RequieredAmmo`)))
  (set `local.RequieredAmmo` (- (`self.MaxMagAmmo`) (`self.CurrentMagAmmo`)))
  (`/Engine/EditorBlueprintResources/StandardMacros.CompareInt` (`self.CurrentClipAmmo`) (`self.MaxMagAmmo`)
    (:`>`
      (set `self.CurrentMagAmmo` (`self.MaxMagAmmo`) :!label _label))
    (:`==`
      (goto _label))
    (:`<`
      (set `self.CurrentMagAmmo` (`KismetMathLibrary.Clamp` (+ (`self.CurrentMagAmmo`) (`self.CurrentClipAmmo`)) 0 (`self.MaxMagAmmo`)))))
  (`/Engine/EditorBlueprintResources/StandardMacros.CompareInt` _returnvalue
    (:`>`
      (set `self.CurrentClipAmmo` _returnvalue))
    (:`==`
      (set `self.CurrentClipAmmo` 0 :!label _label_2))
    (:`<`
      (goto _label_2))))

(fn `UserConstructionScript`
  (`PaperFlipbookComponent.SetFlipbook` (`self.PickupSprite`) (`self.PickupFlipbook`)))
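; BP_Item_Core is an item Blueprint that registers itself toward the player's collectable totals.
; On BeginPlay, if CanCountAsCollectable is set, it casts player 0's character to BP_DefaultCharacter and increments either SecretItemsToCollect or ItemsToCollect, depending on IsSecretItem.
; Each counted item adds itself, so the totals build up from the placed or spawned instances.
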(event `self.ReceiveBeginPlay`
  ;[0 0 0] Set Item Type
  (if (`self.CanCountAsCollectable?`)
    (if (`self.isSecretItem?`)
      (bind _asbp_default_character (cast `/Game/RetroBoomerFPSFramework/Blueprints/Characters/BP_DefaultCharacter` (`GameplayStatics.GetPlayerCharacter` 0)))
      (set `/Game/RetroBoomerFPSFramework/Blueprints/Characters/BP_DefaultCharacter.SecretItemsToCollect` (+ (`/Game/RetroBoomerFPSFramework/Blueprints/Characters/BP_DefaultCharacter.SecretItemsToCollect` _asbp_default_character) 1) _asbp_default_character)
      (else
        (bind _asbp_default_character_2 (cast `/Game/RetroBoomerFPSFramework/Blueprints/Characters/BP_DefaultCharacter` (`GameplayStatics.GetPlayerCharacter` 0)))
        (set `/Game/RetroBoomerFPSFramework/Blueprints/Characters/BP_DefaultCharacter.ItemsToCollect` (+ (`/Game/RetroBoomerFPSFramework/Blueprints/Characters/BP_DefaultCharacter.ItemsToCollect` _asbp_default_character_2) 1) _asbp_default_character_2)))))

(fn `UserConstructionScript`)
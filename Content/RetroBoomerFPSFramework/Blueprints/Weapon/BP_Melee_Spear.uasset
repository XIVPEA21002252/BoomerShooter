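; Spear melee weapon for the retro boomer FPS framework, striking with a short forward reach.
; OnFire sphere-traces on Visibility from above the player's capsule center along the weapon's forward vector, ignoring the armory inventory.
; It applies damage and plays the attack sound at the trace result without checking for a hit, holding IsShooting for the animation's duration.
; A DoOnce reset by a retriggerable delay limits attack rate.
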(event `self.OnFire`
  (bind _returnvalue (+ (`SceneComponent.K2_GetComponentLocation` (`Character.CapsuleComponent` (`self.PlayerCast`))) (0.0 0.0 50.0)))
  ;[0 0 0] Melee Fire Weapon Logic
  (`/Engine/EditorBlueprintResources/StandardMacros.DoOnce` false :!label _label
    (:`Completed`
      (`|ExecutionSequence`
        (:`then_0`
          (set `self.isShooting?` true)
          (bind _outhit (`KismetSystemLibrary.SphereTraceSingle` _returnvalue (+ _returnvalue (* (`KismetMathLibrary.GetForwardVector` (`self.K2_GetActorRotation`)) 250.0)) 20.0 "TraceTypeQuery1" false (`/Game/RetroBoomerFPSFramework/Blueprints/Characters/BP_DefaultCharacter.ArmoryInventory` (`self.PlayerCast`))))
          (bind (_bblockinghit _binitialoverlap _time _distance _location _impactpoint _normal _impactnormal _physmat _hitactor) (`GameplayStatics.BreakHitResult` _outhit))
          (`GameplayStatics.ApplyDamage` _hitactor (`self.WeaponDamage`) null (`self.PlayerCast`))
          (`GameplayStatics.PlaySoundAtLocation` (`self.AttackSound`) _location (struct) 1.0 1.0 0.0 null null null null)
          (`KismetSystemLibrary.Delay` (`self.ShotAnimDuration`))
          (set `self.isShooting?` false))
        (:`then_1`
          (`KismetSystemLibrary.RetriggerableDelay` (`self.DelayBetweenShot`))
          (goto _label :!via `Reset`))))))

(fn `UserConstructionScript`)
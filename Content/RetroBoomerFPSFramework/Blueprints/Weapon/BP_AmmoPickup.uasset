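; Ammo pickup actor shown as a flipbook sprite chosen by AmmoType at construction and yawed each tick toward the player.
; On overlap it tops up a matching equipped weapon's mag, spilling excess into clip ammo.
; Otherwise, given a valid equipped weapon, it searches the armory inventory, writing MaxClipAmmo where that is below CurrentClipAmmo.
; A successful pickup plays a sound, notifies the player and destroys the actor.
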(event `self.ReceiveTick`
  (params (DeltaSeconds :type "Float (single-precision)"))
  (bind (_returnvalue_roll _returnvalue_pitch _returnvalue_yaw) (`KismetMathLibrary.BreakRotator` (`KismetMathLibrary.FindLookAtRotation` (`self.K2_GetActorLocation`) (`self.K2_GetActorLocation` (`GameplayStatics.GetPlayerCharacter` 0)))))
  ;[0 0 0] Sprite Look at Character
  (`SceneComponent.K2_SetWorldRotation` (`self.Arrow`) (`KismetMathLibrary.MakeRotator` 0.0 0.0 _returnvalue_yaw) false false))

(event `self.Sphere.OnComponentBeginOverlap`
  (params (OverlappedComponent :type "PrimitiveComponent Object Reference") (OtherActor :type "Actor Object Reference") (OtherComp :type "PrimitiveComponent Object Reference") (OtherBodyIndex :type Integer) (bFromSweep :type Boolean) (SweepResult :type "HitResult Structure (by ref)"))
  (bind _equipped_weapon (`self.Equipped Weapon`))
  ;[0 0 0] Add ammo to your equipped weapon or inventory weapon
  (bind _asbp_default_character (cast `/Game/RetroBoomerFPSFramework/Blueprints/Characters/BP_DefaultCharacter` OtherActor))
  (bind _output_get (set `self.PlayerCast` _asbp_default_character))
  (bind _equippedweapon (`/Game/RetroBoomerFPSFramework/Blueprints/Characters/BP_DefaultCharacter.EquippedWeapon` _output_get))
  (`/Engine/EditorBlueprintResources/StandardMacros.IsValid` _equippedweapon
    (:`Is Valid`
      (set `self.Equipped Weapon` _equippedweapon)
      (if (and (`|EnumEquality` (`/Game/RetroBoomerFPSFramework/Blueprints/Weapon/Core/BP_Weapon_Core.AmmoType` _equipped_weapon) (`self.AmmoType`)) (or (< (`/Game/RetroBoomerFPSFramework/Blueprints/Weapon/Core/BP_Weapon_Core.CurrentMagAmmo` _equipped_weapon) (`/Game/RetroBoomerFPSFramework/Blueprints/Weapon/Core/BP_Weapon_Core.MaxMagAmmo` _equipped_weapon)) (< (`/Game/RetroBoomerFPSFramework/Blueprints/Weapon/Core/BP_Weapon_Core.CurrentClipAmmo` _equipped_weapon) (`/Game/RetroBoomerFPSFramework/Blueprints/Weapon/Core/BP_Weapon_Core.MaxClipAmmo` _equipped_weapon))))
        (`self.AddWeaponAmmo`)
        (`GameplayStatics.PlaySoundAtLocation` (`self.PickupSound`) (`self.K2_GetActorLocation`) (struct) 1.0 1.0 0.0 null null null null)
        (`/Game/RetroBoomerFPSFramework/Blueprints/Characters/BP_DefaultCharacter.SendNotification` (`self.PlayerCast`) (`|FormatText` "Picked up a Clip (+{amount})" (`self.AddAmmo`)))
        (`self.K2_DestroyActor`)
        (else
          (for _array_element (`/Game/RetroBoomerFPSFramework/Blueprints/Characters/BP_DefaultCharacter.ArmoryInventory` (`self.PlayerCast`))
            (if (and (`|EnumEquality` (`/Game/RetroBoomerFPSFramework/Blueprints/Weapon/Core/BP_Weapon_Core.AmmoType` _array_element) (`self.AmmoType`)) (< (`/Game/RetroBoomerFPSFramework/Blueprints/Weapon/Core/BP_Weapon_Core.MaxClipAmmo` _array_element) (`/Game/RetroBoomerFPSFramework/Blueprints/Weapon/Core/BP_Weapon_Core.CurrentClipAmmo` _array_element)))
              (set `/Game/RetroBoomerFPSFramework/Blueprints/Weapon/Core/BP_Weapon_Core.MaxClipAmmo` (`KismetMathLibrary.Clamp` (+ (`self.AddAmmo`) (`/Game/RetroBoomerFPSFramework/Blueprints/Weapon/Core/BP_Weapon_Core.CurrentMagAmmo` _array_element)) 0 (`/Game/RetroBoomerFPSFramework/Blueprints/Weapon/Core/BP_Weapon_Core.MaxMagAmmo` _array_element)) _array_element)
              (`/Game/RetroBoomerFPSFramework/Blueprints/Characters/BP_DefaultCharacter.SendNotification` (`self.PlayerCast`) (`|FormatText` "Picked up a Clip (+{amount})" (`self.AddAmmo`)))
              (`GameplayStatics.PlaySoundAtLocation` (`self.PickupSound`) (`self.K2_GetActorLocation`) (struct) 1.0 1.0 0.0 null null null null)
              (`self.K2_DestroyActor`)
              (break))))))))

(fn `AddWeaponAmmo`
  (locals (NewMagAmmo :type Integer))
  (bind _equipped_weapon (`self.Equipped Weapon`))
  (set `local.NewMagAmmo` (+ (`self.AddAmmo`) (`/Game/RetroBoomerFPSFramework/Blueprints/Weapon/Core/BP_Weapon_Core.CurrentMagAmmo` _equipped_weapon)))
  (set `/Game/RetroBoomerFPSFramework/Blueprints/Weapon/Core/BP_Weapon_Core.CurrentMagAmmo` (`KismetMathLibrary.Clamp` (`local.NewMagAmmo`) 0 (`/Game/RetroBoomerFPSFramework/Blueprints/Weapon/Core/BP_Weapon_Core.MaxMagAmmo` _equipped_weapon)) _equipped_weapon)
  (if (> (`local.NewMagAmmo`) (`/Game/RetroBoomerFPSFramework/Blueprints/Weapon/Core/BP_Weapon_Core.MaxMagAmmo` _equipped_weapon))
    (set `/Game/RetroBoomerFPSFramework/Blueprints/Weapon/Core/BP_Weapon_Core.CurrentClipAmmo` (`KismetMathLibrary.Clamp` (+ (- (`local.NewMagAmmo`) (`/Game/RetroBoomerFPSFramework/Blueprints/Weapon/Core/BP_Weapon_Core.MaxMagAmmo` _equipped_weapon)) (`/Game/RetroBoomerFPSFramework/Blueprints/Weapon/Core/BP_Weapon_Core.CurrentClipAmmo` _equipped_weapon)) 0 (`/Game/RetroBoomerFPSFramework/Blueprints/Weapon/Core/BP_Weapon_Core.MaxClipAmmo` _equipped_weapon)) _equipped_weapon)))

(fn `SetAmmoType`
  (`PaperFlipbookComponent.SetFlipbook` (`self.PaperFlipbook`) (select `/Game/RetroBoomerFPSFramework/Blueprints/Enums/E_AmmoType` (`self.AmmoType`) :`NewEnumerator0` "/Game/RetroBoomerFPSFramework/Flipbooks/Ammo/FB_Bullet_Revolver.FB_Bullet_Revolver" :`NewEnumerator2` "/Game/RetroBoomerFPSFramework/Flipbooks/Ammo/FB_Bullet_Rifle.FB_Bullet_Rifle" :`NewEnumerator3` "/Game/RetroBoomerFPSFramework/Flipbooks/Ammo/FB_Bullet_Shotgun.FB_Bullet_Shotgun" :`NewEnumerator5` "/Game/RetroBoomerFPSFramework/Flipbooks/Ammo/FB_Bullet_RPG.FB_Bullet_RPG" :!type "PaperFlipbook Object Reference")))

(fn `UserConstructionScript`
  (`self.SetAmmoType`))
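; BP_SecretEntrance is an interactable secret door that slides to a relative destination when opened.
; OpenSecret adds the destination as a control point and activates an InterpToMovement component, whose duration comes from the construction script, along with a moving sound.
; When movement stops, the audio fades out and the wall's collision is disabled.
; GetActorData reports only the interactable flag, with blank title and zero health.
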(event `OpenSecret`
  (bind _interptomovement (`self.InterpToMovement`))
  ;[0 0 0] Secret Actor Interaction
  ;;[0.0999 0.0999 0.0999] Handles secret doors by moving them to a target destination and activating audio feedback when the player triggers the secret.
  (`InterpToMovementComponent.AddControlPointPosition` _interptomovement (`self.Destination`) true)
  (`ActorComponent.SetActive` _interptomovement true true)
  (`ActorComponent.SetActive` (`self.AudioMoving`) true true))

(event `self.InterpToMovement.OnInterpToStop`
  (params (ImpactResult :type "HitResult Structure (by ref)") (Time :type "Float (single-precision)"))
  ;[0 0 0] Secret Actor Interaction
  ;;[0.0999 0.0999 0.0999] On Movement Finish
  (`AudioComponent.FadeOut` (`self.AudioMoving`) 0.2 0.0 "Linear")
  (`PrimitiveComponent.SetCollisionEnabled` (`self.Wall`) "NoCollision"))

(fn `GetActorData`
  (returns (`isInteractable?` :type Boolean) (TextTitle :type Text) (CurHealth :type "Float (double-precision)") (MaxHealth :type "Float (double-precision)"))
  (return (`self.Is Interactable?`) "" 0.0 0.0))

(fn `UserConstructionScript`
  (set `InterpToMovementComponent.Duration` (`self.MovementDuration`) (`self.InterpToMovement`)))
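; BP_HealthPickup is a health pickup for the retro boomer FPS that restores health to the player character on touch.
; Each tick, its Arrow component yaws toward player 0 so the sprite faces the player.
; Sphere overlap by BP_DefaultCharacter, if below max health, passes the pickup's Health to ACHealth.SetHealth, triggers green feedback, a notification and a sound, then destroys the actor.
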(event `self.ReceiveTick`
  (params (DeltaSeconds :type "Float (single-precision)"))
  (bind (_returnvalue_roll _returnvalue_pitch _returnvalue_yaw) (`KismetMathLibrary.BreakRotator` (`KismetMathLibrary.FindLookAtRotation` (`self.K2_GetActorLocation`) (`self.K2_GetActorLocation` (`GameplayStatics.GetPlayerCharacter` 0)))))
  ;[0 0 0] Sprite Look at Character
  (`SceneComponent.K2_SetWorldRotation` (`self.Arrow`) (`KismetMathLibrary.MakeRotator` 0.0 0.0 _returnvalue_yaw) false false))

(event `self.Sphere.OnComponentBeginOverlap`
  (params (OverlappedComponent :type "PrimitiveComponent Object Reference") (OtherActor :type "Actor Object Reference") (OtherComp :type "PrimitiveComponent Object Reference") (OtherBodyIndex :type Integer) (bFromSweep :type Boolean) (SweepResult :type "HitResult Structure (by ref)"))
  ;[0 0 0] Add health
  (bind _asbp_default_character (cast `/Game/RetroBoomerFPSFramework/Blueprints/Characters/BP_DefaultCharacter` OtherActor))
  (bind _ac_health (`/Game/RetroBoomerFPSFramework/Blueprints/Characters/BP_CharacterCore.AC_Health` _asbp_default_character))
  (if (< (`/Game/RetroBoomerFPSFramework/Blueprints/ActorComponents/AC_Health.Health` _ac_health) (`/Game/RetroBoomerFPSFramework/Blueprints/ActorComponents/AC_Health.MaxHealth` _ac_health))
    (`/Game/RetroBoomerFPSFramework/Blueprints/ActorComponents/AC_Health.Set_Health` _ac_health (`self.Health`))
    (`/Game/RetroBoomerFPSFramework/Blueprints/Characters/BP_DefaultCharacter.FeedbackPickup` _asbp_default_character (struct :`R` 0.012286 :`G` 1.0 :`A` 1.0))
    (`/Game/RetroBoomerFPSFramework/Blueprints/Characters/BP_DefaultCharacter.SendNotification` _asbp_default_character (`|FormatText` "Picked up a Health (+{Health})" (`self.Health`)))
    (`GameplayStatics.PlaySoundAtLocation` "/Game/RetroBoomerFPSFramework/Sounds/SFX/General/Cue/Cue_Healthpotion.Cue_Healthpotion" (`self.K2_GetActorLocation`) (struct) 1.0 1.0 0.0 null null null null)
    (`self.K2_DestroyActor`)))

(fn `UserConstructionScript`)
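; BP_Target is a damageable moving target actor.
; On BeginPlay it adds a relative Destination control point to its Movement component, defining the path it travels.
; Damage goes through the ACHealth component, and health is reset to a fixed value whenever ApplyDamage returns true, so the target is reusable.
; GetActorData reports it as a non-interactable "Target" with current and maximum health.
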(event `self.ReceiveBeginPlay`
  ;[0 0 0] Beginplay
  (`InterpToMovementComponent.AddControlPointPosition` (`self.Movement`) (`self.Destination`) true))

(event `self.ReceiveAnyDamage`
  (params (Damage :type "Float (single-precision)") (DamageType :type "DamageType Object Reference") (InstigatedBy :type "Controller Object Reference") (DamageCauser :type "Actor Object Reference"))
  ;[0 0 0] AnyDamage
  (bind _dead (`/Game/RetroBoomerFPSFramework/Blueprints/ActorComponents/AC_Health.ApplyDamage` (`self.AC_Health`) Damage))
  (if _dead
    (`/Game/RetroBoomerFPSFramework/Blueprints/ActorComponents/AC_Health.Set_Health` (`self.AC_Health`) 100.0)))

(fn `GetActorData`
  (returns (`isInteractable?` :type Boolean) (TextTitle :type Text) (CurHealth :type "Float (double-precision)") (MaxHealth :type "Float (double-precision)"))
  (bind _ac_health (`self.AC_Health`))
  (return false "Target" (`/Game/RetroBoomerFPSFramework/Blueprints/ActorComponents/AC_Health.Health` _ac_health) (`/Game/RetroBoomerFPSFramework/Blueprints/ActorComponents/AC_Health.MaxHealth` _ac_health)))

(fn `UserConstructionScript`)
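; BP_ArmorPickup is an armor pickup that grants its Armor value to the player character on contact.
; Each tick it yaws an Arrow component toward player 0 so the sprite faces the player.
; Sphere overlap with a BP_DefaultCharacter below max armor calls SetArmor on its ACHealth component.
; It then triggers blue pickup feedback, a notification and a sound before destroying itself.
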(event `self.ReceiveTick`
  (params (DeltaSeconds :type "Float (single-precision)"))
  (bind (_returnvalue_roll _returnvalue_pitch _returnvalue_yaw) (`KismetMathLibrary.BreakRotator` (`KismetMathLibrary.FindLookAtRotation` (`self.K2_GetActorLocation`) (`self.K2_GetActorLocation` (`GameplayStatics.GetPlayerCharacter` 0)))))
  ;[0 0 0] Sprite Look at Character
  (`SceneComponent.K2_SetWorldRotation` (`self.Arrow`) (`KismetMathLibrary.MakeRotator` 0.0 0.0 _returnvalue_yaw) false false))

(event `self.Sphere.OnComponentBeginOverlap`
  (params (OverlappedComponent :type "PrimitiveComponent Object Reference") (OtherActor :type "Actor Object Reference") (OtherComp :type "PrimitiveComponent Object Reference") (OtherBodyIndex :type Integer) (bFromSweep :type Boolean) (SweepResult :type "HitResult Structure (by ref)"))
  ;[0 0 0] Add armor to the character
  (bind _asbp_default_character (cast `/Game/RetroBoomerFPSFramework/Blueprints/Characters/BP_DefaultCharacter` OtherActor))
  (bind _ac_health (`/Game/RetroBoomerFPSFramework/Blueprints/Characters/BP_CharacterCore.AC_Health` _asbp_default_character))
  (if (< (`/Game/RetroBoomerFPSFramework/Blueprints/ActorComponents/AC_Health.Armor` _ac_health) (`/Game/RetroBoomerFPSFramework/Blueprints/ActorComponents/AC_Health.MaxArmor` _ac_health))
    (`/Game/RetroBoomerFPSFramework/Blueprints/ActorComponents/AC_Health.Set_Armor` _ac_health (`self.Armor`))
    (`/Game/RetroBoomerFPSFramework/Blueprints/Characters/BP_DefaultCharacter.FeedbackPickup` _asbp_default_character (struct :`G` 0.095457 :`B` 1.0 :`A` 1.0))
    (`/Game/RetroBoomerFPSFramework/Blueprints/Characters/BP_DefaultCharacter.SendNotification` _asbp_default_character (`|FormatText` "Picked up Armor (+{armor})" (`self.Armor`)))
    (`GameplayStatics.PlaySoundAtLocation` "/Game/RetroBoomerFPSFramework/Sounds/SFX/General/Cue/Cue_GameArmorOn.Cue_GameArmorOn" (`self.K2_GetActorLocation`) (struct) 1.0 1.0 0.0 null null null null)
    (`self.K2_DestroyActor`)))

(fn `UserConstructionScript`)
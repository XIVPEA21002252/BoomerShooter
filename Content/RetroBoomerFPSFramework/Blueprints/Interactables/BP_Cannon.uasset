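; BP_Cannon is an automatic cannon hazard that repeatedly fires fireball projectiles.
; On BeginPlay it starts a looping timer with a random period picked once, so each cannon keeps its own steady rhythm.
; Each shot switches to the firing flipbook, plays a sound and spawns a BP_EnemyProjectile from the Arrow component with the cannon's damage and damage type.
; A short delay then restores the idle flipbook.
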(event `self.ReceiveBeginPlay`
  ;[0 0 0] Automatically fires projectiles at random intervals. It changes the flipbook animation, plays a firing sound, spawns a projectile from an arrow location with defined damage, waits briefly, and then resets the flipbook.
  (`KismetSystemLibrary.K2_SetTimerDelegate` (delegate `FireCannon`) (`KismetMathLibrary.RandomFloatInRange` 1.0 2.0) true))

(event `FireCannon`
  ;[0 0 0] Automatically fires projectiles at random intervals. It changes the flipbook animation, plays a firing sound, spawns a projectile from an arrow location with defined damage, waits briefly, and then resets the flipbook.
  (`PaperFlipbookComponent.SetFlipbook` (`self.PaperFlipbook`) "/Game/RetroBoomerFPSFramework/Flipbooks/Props/FB_Cannon_Fire.FB_Cannon_Fire")
  (`GameplayStatics.PlaySoundAtLocation` "/Game/RetroBoomerFPSFramework/Sounds/SFX/General/Cue/Cue_cannonfire5.Cue_cannonfire5" (`self.K2_GetActorLocation`) (struct) 1.0 1.0 0.0 null null null null)
  (`|SpawnActorFromClass` "/Game/RetroBoomerFPSFramework/Blueprints/Projectiles/BP_EnemyProjectile.BP_EnemyProjectile_C" (`SceneComponent.K2_GetComponentToWorld` (`self.Arrow`)) "AlwaysSpawn" "OverrideRootScale" null (`self.Damage`) "/Game/RetroBoomerFPSFramework/Flipbooks/Props/FB_Fireball.FB_Fireball" "/Game/RetroBoomerFPSFramework/Blueprints/DamageType/DAT_Cannon.DAT_Cannon_C" null)
  (`KismetSystemLibrary.Delay` 0.46)
  (`PaperFlipbookComponent.SetFlipbook` (`self.PaperFlipbook`) "/Game/RetroBoomerFPSFramework/Flipbooks/Props/FB_Cannon_Idle.FB_Cannon_Idle"))

(fn `UserConstructionScript`)
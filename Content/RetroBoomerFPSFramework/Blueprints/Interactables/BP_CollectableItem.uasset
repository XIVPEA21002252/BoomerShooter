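; Collectable pickup for the retro boomer shooter, configured by IsSecretItem as either a purple gem or a secret magic book.
; The construction script sets the flipbook and scale for that type, and Tick yaws the arrow component toward the player for a billboard sprite effect.
; On sphere overlap by BP_DefaultCharacter, a DoOnce increments the player's matching item counter, sends a notification, plays a sound and destroys the actor.
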(event `self.ReceiveTick`
  (params (DeltaSeconds :type "Float (single-precision)"))
  (bind (_returnvalue_roll _returnvalue_pitch _returnvalue_yaw) (`KismetMathLibrary.BreakRotator` (`KismetMathLibrary.FindLookAtRotation` (`self.K2_GetActorLocation`) (`self.K2_GetActorLocation` (`GameplayStatics.GetPlayerCharacter` 0)))))
  ;[0 0 0] Sprite Look at Character
  (`SceneComponent.K2_SetWorldRotation` (`self.Arrow_0`) (`KismetMathLibrary.MakeRotator` 0.0 0.0 _returnvalue_yaw) false false))

(event `self.Sphere.OnComponentBeginOverlap`
  (params (OverlappedComponent :type "PrimitiveComponent Object Reference") (OtherActor :type "Actor Object Reference") (OtherComp :type "PrimitiveComponent Object Reference") (OtherBodyIndex :type Integer) (bFromSweep :type Boolean) (SweepResult :type "HitResult Structure (by ref)"))
  ;[0 0 0] handles item pickups. When the player overlaps, it checks if the item is a secret or a regular pickup, updates the player’s collected count, sends a notification, plays a sound, and then destroys the pickup actor.
  (bind _asbp_default_character (cast `/Game/RetroBoomerFPSFramework/Blueprints/Characters/BP_DefaultCharacter` OtherActor))
  (set `self.PlayerCast` _asbp_default_character)
  (`/Engine/EditorBlueprintResources/StandardMacros.DoOnce` false
    (:`Completed`
      (if (`self.isSecretItem?`)
        (`/Engine/EditorBlueprintResources/StandardMacros.IncrementInt` (`/Game/RetroBoomerFPSFramework/Blueprints/Characters/BP_DefaultCharacter.SecretItemsCollected` (`self.PlayerCast`))
          (:`  `
            (`/Game/RetroBoomerFPSFramework/Blueprints/Characters/BP_DefaultCharacter.SendNotification` (`self.PlayerCast`) (`|FormatText` "Secret Found!"))
            (`GameplayStatics.PlaySoundAtLocation` "/Game/RetroBoomerFPSFramework/Sounds/SFX/General/Cue/Cue_ClueFound1.Cue_ClueFound1" (`self.K2_GetActorLocation`) (struct) 1.0 1.0 0.0 null null null null)))
        (else
          (`/Engine/EditorBlueprintResources/StandardMacros.IncrementInt` (`/Game/RetroBoomerFPSFramework/Blueprints/Characters/BP_DefaultCharacter.ItemsCollected` (`self.PlayerCast`))
            (:`  `
              (`/Game/RetroBoomerFPSFramework/Blueprints/Characters/BP_DefaultCharacter.SendNotification` (`self.PlayerCast`) (`|FormatText` "Purple Gem"))
              (`GameplayStatics.PlaySoundAtLocation` "/Game/RetroBoomerFPSFramework/Sounds/SFX/General/Wav/Wave_Bonus.Wave_Bonus" (`self.K2_GetActorLocation`) (struct) 1.0 1.0 0.0 null null null null)))))
      (`self.K2_DestroyActor`))))

(fn `UserConstructionScript`
  (`parent.UserConstructionScript`)
  (if (`self.isSecretItem?`)
    (`SceneComponent.SetWorldScale3D` (`self.FP_Item`) (0.2 0.2 0.2))
    (`PaperFlipbookComponent.SetFlipbook` (`self.FP_Item`) "/Game/RetroBoomerFPSFramework/Flipbooks/Props/FB_MagicBook.FB_MagicBook")
    (else
      (`SceneComponent.SetWorldScale3D` (`self.FP_Item`) (1.8 1.8 1.8))
      (`PaperFlipbookComponent.SetFlipbook` (`self.FP_Item`) "/Game/RetroBoomerFPSFramework/Flipbooks/Props/FB_Gem.FB_Gem"))))
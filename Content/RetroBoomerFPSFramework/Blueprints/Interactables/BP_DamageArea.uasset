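; BP_DamageArea is a hazard floor, such as acid, that repeatedly damages the player standing on it.
; Overlapping the Damage component caches the living BP_CharacterCore, applies damage immediately and starts a looping DoDamage timer at DamageInterval.
; Leaving only clears the cached reference, so the timer stops itself on its next tick, and damage skips dead players.
; The construction script applies DamageFloorMaterial to the Cube.
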(event `self.Damage.OnComponentBeginOverlap`
  (params (OverlappedComponent :type "PrimitiveComponent Object Reference") (OtherActor :type "Actor Object Reference") (OtherComp :type "PrimitiveComponent Object Reference") (OtherBodyIndex :type Integer) (bFromSweep :type Boolean) (SweepResult :type "HitResult Structure (by ref)"))
  ;[0 0 0] Deals damage to the player while standing on the acid, triggering every DamageInterval seconds until they leave.
  (bind _asbp_character_core (cast `/Game/RetroBoomerFPSFramework/Blueprints/Characters/BP_CharacterCore` OtherActor))
  (bind _output_get (set `self.PlayerCast` _asbp_character_core))
  (if (not (`/Game/RetroBoomerFPSFramework/Blueprints/Characters/BP_CharacterCore.isDead?` _output_get))
    (`self.DoDamage`)
    (`KismetSystemLibrary.K2_SetTimer` null "DoDamage" (`self.DamageInterval`) true)
    (else
      (`KismetSystemLibrary.K2_ClearTimer` null "DoDamage"))))

(event `self.Damage.OnComponentEndOverlap`
  (params (OverlappedComponent :type "PrimitiveComponent Object Reference") (OtherActor :type "Actor Object Reference") (OtherComp :type "PrimitiveComponent Object Reference") (OtherBodyIndex :type Integer))
  ;[0 0 0] Deals damage to the player while standing on the acid, triggering every DamageInterval seconds until they leave.
  (set `self.PlayerCast` null))

(fn `DoDamage`
  (bind _playercast (`self.PlayerCast`))
  (`/Engine/EditorBlueprintResources/StandardMacros.IsValid` _playercast
    (:`Is Valid`
      (if (not (`/Game/RetroBoomerFPSFramework/Blueprints/Characters/BP_CharacterCore.isDead?` _playercast))
        (`GameplayStatics.ApplyDamage` (`self.PlayerCast`) (`self.Base Damage`) null self (`self.Damage Type Class`))))
    (:`Is Not Valid`
      (`KismetSystemLibrary.K2_ClearTimer` null "DoDamage"))))

(fn `UserConstructionScript`
  (`PrimitiveComponent.SetMaterial` (`self.Cube`) 0 (`self.DamageFloorMaterial`)))
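; BP_Explosion is a short-lived explosion actor that shows a flipbook sprite and damages nearby actors.
; On BeginPlay it sets its Paper2D flipbook, applies radial damage with falloff using configurable damage, radii, origin and ignore list, then destroys itself after a delay.
; Each tick it yaws toward the player pawn, so the flat sprite acts as a billboard locked to the vertical axis.
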(event `self.ReceiveBeginPlay`
  ;[0 0 0] Beginplay - It sets the explosion flipbook, applies radial damage with falloff to nearby actors, waits for the explosion duration, and then destroys itself.
  (`PaperFlipbookComponent.SetFlipbook` (`self.PaperFlipbook`) (`self.New Flipbook`))
  (`GameplayStatics.ApplyRadialDamageWithFalloff` (`self.ExplosionDamage`) (`self.ExplosionMinDamage`) (`self.ExplosionLoc`) (`self.ExplosionInnerRadius`) (`self.ExplosionOuterRadius`) (`self.ExplosionDamageFalloff`) (`self.Damage Type Class`) (`self.Ignore Actors`) (`self.Damage Causer`) null)
  (`KismetSystemLibrary.Delay` (`self.ExplosionDuration`))
  (`self.K2_DestroyActor`))

(event `self.ReceiveTick`
  (params (DeltaSeconds :type "Float (single-precision)"))
  (bind (_returnvalue_roll _returnvalue_pitch _returnvalue_yaw) (`KismetMathLibrary.BreakRotator` (`KismetMathLibrary.FindLookAtRotation` (`self.K2_GetActorLocation`) (`self.K2_GetActorLocation` (`GameplayStatics.GetPlayerPawn` 0)))))
  ;[0 0 0] Tick Event - Sprite look at character
  (`self.K2_SetActorRotation` (`KismetMathLibrary.MakeRotator` 0.0 0.0 _returnvalue_yaw)))

(fn `UserConstructionScript`)
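; BP_Barrel is a sprite-based explosive barrel that detonates after taking lethal damage.
; Damage feeds the AC Health component; on death it disables collision and shows a pulsing radius decal through a delay, with Tick keeping the decal on the barrel.
; It then spawns BP_Explosion with its damage settings, plays sound and optional camera shake, and either swaps to a destroyed sprite or destroys itself.
; GetActorData reports name and health as non-interactable.
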(event `self.ReceiveTick`
  (params (DeltaSeconds :type "Float (single-precision)"))
  ;[0 0 0] Event Tick
  (`parent.ReceiveTick` DeltaSeconds)
  ;;[0.01096 0.01096 0.01096] Move the decal with the barrel - tick only active after barrel starts burning
  (bind _decalcomponent (`self.DecalComponent`)
    (:`then`
      (`SceneComponent.K2_SetWorldLocation` _decalcomponent (`self.K2_GetActorLocation`) false false))
    (:`else`)))

(event `self.ReceiveBeginPlay`
  (bind _ac_health (`self.AC_Health`))
  ;[0 0 0] Beginplay - sets the actor’s Health and Max Health based on the AC Health value, ensuring the actor starts with its defined full health.
  (bind _output_get (set `/Game/RetroBoomerFPSFramework/Blueprints/ActorComponents/AC_Health.Health` (`self.Health`) _ac_health))
  (set `/Game/RetroBoomerFPSFramework/Blueprints/ActorComponents/AC_Health.MaxHealth` _output_get _ac_health))

(event `self.ReceiveAnyDamage`
  (params (Damage :type "Float (single-precision)") (DamageType :type "DamageType Object Reference") (InstigatedBy :type "Controller Object Reference") (DamageCauser :type "Actor Object Reference"))
  (bind _explosion_outer_radius (`self.Explosion Outer Radius`))
  (bind _returnvalue (`SceneComponent.K2_GetComponentLocation` (`self.Collision`)))
  ;[0 0 0] Any Damage - applies damage, spawns decal + explosion actor, plays sound/camera shake, disables collision, and destroys actor
  (if (not (`self.isDestroy?`))
    (bind _dead (`/Game/RetroBoomerFPSFramework/Blueprints/ActorComponents/AC_Health.ApplyDamage` (`self.AC_Health`) Damage))
    (bind _output_get (set `self.isDestroy?` _dead))
    (if _output_get
      (bind _returnvalue_2 (`GameplayStatics.SpawnDecalAtLocation` "/Game/RetroBoomerFPSFramework/Materials/Decal/MI_PulseCircle.MI_PulseCircle" (`KismetMathLibrary.MakeVector` 5.0 _explosion_outer_radius _explosion_outer_radius) (`self.K2_GetActorLocation`) (struct :`Pitch` 90.0) (`self.DelayBeforeExplode`)))
      (set `self.DecalComponent` _returnvalue_2)
      (`PrimitiveComponent.SetCollisionEnabled` (`self.Collision`) "NoCollision")
      (`KismetSystemLibrary.Delay` (`self.DelayBeforeExplode`))
      (`|SpawnActorFromClass` "/Game/RetroBoomerFPSFramework/Blueprints/Interactables/BP_Explosion.BP_Explosion_C" (`KismetMathLibrary.MakeTransform` _returnvalue) "Undefined" "OverrideRootScale" null (`self.ExplosionFlipbook`) (`self.ExplosionDamage`) (`self.Explosion Min Damage`) (`self.K2_GetActorLocation`) (`self.Explosion Inner Radius`) (`self.Explosion Outer Radius`) (`self.Explosion Damage Falloff`) 0.5 self (`self.Damage Type Class`) null)
      (if (`self.CameraShake?`)
        (`GameplayStatics.PlayWorldCameraShake` (`self.CameraShake`) _returnvalue 500.0 5000.0 1.0 true))
      (`GameplayStatics.PlaySoundAtLocation` (`self.Explosion_Sound`) _returnvalue (struct) 1.0 1.0 0.0 null null null null)
      (if (`self.UseDestroySprite?`)
        (`PaperSpriteComponent.SetSprite` (`self.PaperSprite`) (`self.Destroyed_Sprite`))
        (else
          (`self.K2_DestroyActor`)))
      (bind _decalcomponent (`self.DecalComponent`)
        (:`then`
          (`ActorComponent.K2_DestroyComponent` _decalcomponent))
        (:`else`)))))

(fn `GetActorData`
  (returns (`isInteractable?` :type Boolean) (TextTitle :type Text) (CurHealth :type "Float (double-precision)") (MaxHealth :type "Float (double-precision)"))
  (bind _ac_health (`self.AC_Health`))
  (return false (`self.Display Name`) (`/Game/RetroBoomerFPSFramework/Blueprints/ActorComponents/AC_Health.Health` _ac_health) (`/Game/RetroBoomerFPSFramework/Blueprints/ActorComponents/AC_Health.MaxHealth` _ac_health)))

(fn `UserConstructionScript`
  (`PaperSpriteComponent.SetSprite` (`self.PaperSprite`) (`self.IdleSprite`)))
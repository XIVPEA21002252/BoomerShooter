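; BP_Lever is an interactable lever that unlocks a linked door.
; On interaction it plays a lever sound, disables collision on its paper sprite and swaps it to the switched-off sprite, then clears the NeedKey flag on DoorToOpen if that reference is valid.
; GetActorData reports its interactable flag and prompt text, with health values fixed at zero.
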(event `InteractLever`
  (bind _doortoopen (`self.DoorToOpen`))
  ;[0 0 0] Interact with Lever
  (`GameplayStatics.PlaySoundAtLocation` "/Game/RetroBoomerFPSFramework/Sounds/SFX/General/Cue/Cue_Lever.Cue_Lever" (`self.K2_GetActorLocation`) (struct) 1.0 1.0 0.0 null null null null)
  (`PrimitiveComponent.SetCollisionEnabled` (`self.PaperSprite`) "NoCollision")
  (`PaperSpriteComponent.SetSprite` (`self.PaperSprite`) "/Game/RetroBoomerFPSFramework/Sprites/SP_switch-off_Sprite.SP_switch-off_Sprite")
  (`/Engine/EditorBlueprintResources/StandardMacros.IsValid` _doortoopen
    (:`Is Valid`
      (set `/Game/RetroBoomerFPSFramework/Blueprints/Interactables/BP_Door.NeedKey?` false _doortoopen))))

(fn `GetActorData`
  (returns (`isInteractable?` :type Boolean) (TextTitle :type Text) (CurHealth :type "Float (double-precision)") (MaxHealth :type "Float (double-precision)"))
  (return (`self.Is Interactable?`) (`self.InteractText`) 0.0 0.0))

(fn `UserConstructionScript`)
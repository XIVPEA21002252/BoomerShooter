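; BP_LevelComplete is a finish trigger that ends the level when the player overlaps its box.
; The overlap fires once for BP_DefaultCharacter and creates WB_LevelResults from the character's secrets, enemies, items and start time stats.
; It then adds the widget to the viewport, pauses the game and plays a 2D completion sound.
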(event `self.Box.OnComponentBeginOverlap`
  (params (OverlappedComponent :type "PrimitiveComponent Object Reference") (OtherActor :type "Actor Object Reference") (OtherComp :type "PrimitiveComponent Object Reference") (OtherBodyIndex :type Integer) (bFromSweep :type Boolean) (SweepResult :type "HitResult Structure (by ref)"))
  ;[0 0 0] Triggers the end of the level when the player overlaps the finish box, showing the results widget with stats, pausing the game, and playing the victory sound.
  (bind _asbp_default_character (cast `/Game/RetroBoomerFPSFramework/Blueprints/Characters/BP_DefaultCharacter` OtherActor))
  (`/Engine/EditorBlueprintResources/StandardMacros.DoOnce` false
    (:`Completed`
      (bind _returnvalue (`|CreateWidget` "/Game/RetroBoomerFPSFramework/Blueprints/Widgets/Gameplay/WB_LevelResults.WB_LevelResults_C" null (`/Game/RetroBoomerFPSFramework/Blueprints/Characters/BP_DefaultCharacter.SecretItemsCollected` _asbp_default_character) (`/Game/RetroBoomerFPSFramework/Blueprints/Characters/BP_DefaultCharacter.SecretItemsToCollect` _asbp_default_character) (`/Game/RetroBoomerFPSFramework/Blueprints/Characters/BP_DefaultCharacter.EnemiesDefeated` _asbp_default_character) (`/Game/RetroBoomerFPSFramework/Blueprints/Characters/BP_DefaultCharacter.EnemiesToDefeat` _asbp_default_character) (`/Game/RetroBoomerFPSFramework/Blueprints/Characters/BP_DefaultCharacter.ItemsCollected` _asbp_default_character) (`/Game/RetroBoomerFPSFramework/Blueprints/Characters/BP_DefaultCharacter.ItemsToCollect` _asbp_default_character) (`/Game/RetroBoomerFPSFramework/Blueprints/Characters/BP_DefaultCharacter.StartTime` _asbp_default_character)))
      (`UserWidget.AddToViewport` _returnvalue 0)
      (`GameplayStatics.SetGamePaused` true)
      (`GameplayStatics.PlaySound2D` "/Game/RetroBoomerFPSFramework/Sounds/SFX/General/Cue/Cue_FantasyGameDarkLevelUnlock.Cue_FantasyGameDarkLevelUnlock" 1.0 1.0 0.0 null null))))

(fn `UserConstructionScript`)
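; BP_KeyPickup is a colored key pickup, shown as a sprite, that the player collects by touching it.
; The construction script picks the blue, red or yellow flipbook from KeyColor.
; Tick yaws the Arrow component toward the player as a billboard effect.
; When BP_DefaultCharacter overlaps the Sphere, it receives the key and a notification, a sound plays, and the pickup destroys itself.
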(event `self.ReceiveTick`
  (params (DeltaSeconds :type "Float (single-precision)"))
  (bind (_returnvalue_roll _returnvalue_pitch _returnvalue_yaw) (`KismetMathLibrary.BreakRotator` (`KismetMathLibrary.FindLookAtRotation` (`self.K2_GetActorLocation`) (`self.K2_GetActorLocation` (`GameplayStatics.GetPlayerCharacter` 0)))))
  ;[0 0 0] Sprite Look at Character
  (`SceneComponent.K2_SetWorldRotation` (`self.Arrow`) (`KismetMathLibrary.MakeRotator` 0.0 0.0 _returnvalue_yaw) false false))

(event `self.Sphere.OnComponentBeginOverlap`
  (params (OverlappedComponent :type "PrimitiveComponent Object Reference") (OtherActor :type "Actor Object Reference") (OtherComp :type "PrimitiveComponent Object Reference") (OtherBodyIndex :type Integer) (bFromSweep :type Boolean) (SweepResult :type "HitResult Structure (by ref)"))
  (bind _keycolor (`self.KeyColor`))
  ;[0 0 0] Add key to the character
  (bind _asbp_default_character (cast `/Game/RetroBoomerFPSFramework/Blueprints/Characters/BP_DefaultCharacter` OtherActor))
  (`/Game/RetroBoomerFPSFramework/Blueprints/Characters/BP_DefaultCharacter.AddKey` _asbp_default_character _keycolor)
  (`/Game/RetroBoomerFPSFramework/Blueprints/Characters/BP_DefaultCharacter.SendNotification` _asbp_default_character (`|FormatText` "Picked up the {KeyColor} Key!" (`|GetEnumeratorNameAsString` _keycolor)))
  (`GameplayStatics.PlaySoundAtLocation` "/Game/RetroBoomerFPSFramework/Sounds/SFX/General/Cue/Cue_treasure-found.Cue_treasure-found" (`self.K2_GetActorLocation`) (struct) 1.0 1.0 0.0 null null null null)
  (`self.K2_DestroyActor`))

(fn `UserConstructionScript`
  (`PaperFlipbookComponent.SetFlipbook` (`self.PaperFlipbook`) (select `/Game/RetroBoomerFPSFramework/Blueprints/Enums/E_KeyItems` (`self.KeyColor`) :`NewEnumerator0` "/Game/RetroBoomerFPSFramework/Flipbooks/Keys/FB_KeyBlue.FB_KeyBlue" :`NewEnumerator1` "/Game/RetroBoomerFPSFramework/Flipbooks/Keys/FB_KeyRed.FB_KeyRed" :`NewEnumerator2` "/Game/RetroBoomerFPSFramework/Flipbooks/Keys/FB_KeyYellow.FB_KeyYellow" :!type "PaperFlipbook Object Reference")))